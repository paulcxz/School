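; Stage lighting rig for a lecture hall, with two rows of top lights plus DMX wash LEDs and moving heads.
; The construction script gathers child-actor fixtures into arrays, evenly spaces each row and assigns a dynamic emissive material per top-light row.
; BeginPlay pushes preset normalized DMX attribute values to the moving heads.
; CE_TurnOn and CE_TurnOff switch only the rect light and first row's material intensity.
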(event Custom|CE_TurnOff
  (Rendering|Components|Light|SetIntensity (Variables|Default|GetRectLight) 0.0)
  (Rendering|Material|SetScalarParameterValue (Variables|Default|GetMI_Light_Line1) "Intensity" 0.0 :!class /Script/Engine.MaterialInstanceDynamic))

(event Custom|CE_TurnOn
  (Rendering|Components|Light|SetIntensity (Variables|Default|GetRectLight) (Variables|Default|GetIntensity))
  (Rendering|Material|SetScalarParameterValue (Variables|Default|GetMI_Light_Line1) "Intensity" 15.0 :!class /Script/Engine.MaterialInstanceDynamic))

(event EventBeginPlay
  (Class|DMXFixtureActor|PushNormalizedValuesPerAttribute (Variables|Default|GetMovingHeadsL2) (Utilities|Struct|MakeDMXNormalizedAttributeValueMap (Utilities|Map|MakeMap "(Name=\"Red\")" 16.0 "(Name=\"Green\")" 0.0 "(Name=\"Blue\")" 0.0 "(Name=\"Dimmer\")" 0.2))))

(event Collision|EventActorBeginOverlap
  (params (OtherActor :type Actor%20Object%20Reference)))

(event EventTick
  (params (DeltaSeconds :type Float%20%28single-precision%29)))

(fn ConstructionScript
  (Utilities|FlowControl|Sequence
    (:then_0
      (bind _returnvalue (Rendering|Material|CreateDynamicMaterialInstance "/Game/Hollywood_Vol3/Materials/Instances/MI_Light_Stand_01a.MI_Light_Stand_01a" "None" "None" :!class /Script/Engine.KismetMaterialLibrary))
      (Variables|Default|SetMI_Light_Line1 _returnvalue)
      (bind _returnvalue_2 (Rendering|Material|CreateDynamicMaterialInstance "/Game/Hollywood_Vol3/Materials/Instances/MI_Light_Stand_01a.MI_Light_Stand_01a" "None" "None" :!class /Script/Engine.KismetMaterialLibrary))
      (Variables|Default|SetMI_Light_Line2 _returnvalue_2)
      (Variables|Default|SetSM_TopLightLine2 (Utilities|Array|MakeArray (Variables|Default|GetTopLightHead15) (Variables|Default|GetTopLightHead16) (Variables|Default|GetTopLightHead9) (Variables|Default|GetTopLightHead10) (Variables|Default|GetTopLightHead13) (Variables|Default|GetTopLightHead11) (Variables|Default|GetTopLightHead12) (Variables|Default|GetTopLightHead14)))
      (Variables|Default|SetSM_TopLightLine1 (Utilities|Array|MakeArray (Variables|Default|GetTopLightHead2) (Variables|Default|GetTopLightHead1) (Variables|Default|GetTopLightHead8) (Variables|Default|GetTopLightHead7) (Variables|Default|GetTopLightHead5) (Variables|Default|GetTopLightHead4) (Variables|Default|GetTopLightHead6) (Variables|Default|GetTopLightHead3)))
      (Variables|Default|SetWashLEDsL1 (Utilities|Array|MakeArray (.AsBP%20Wash%20LEDCXZ (Utilities|Casting|CastToBP_WashLEDCXZ (Variables|/Script/Engine.ChildActorComponent|GetChildActor (Variables|Default|GetLine1WashLED2)))) (.AsBP%20Wash%20LEDCXZ (Utilities|Casting|CastToBP_WashLEDCXZ (Variables|/Script/Engine.ChildActorComponent|GetChildActor (Variables|Default|GetLine1WashLED8)))) (.AsBP%20Wash%20LEDCXZ (Utilities|Casting|CastToBP_WashLEDCXZ (Variables|/Script/Engine.ChildActorComponent|GetChildActor (Variables|Default|GetLine1WashLED9)))) (.AsBP%20Wash%20LEDCXZ (Utilities|Casting|CastToBP_WashLEDCXZ (Variables|/Script/Engine.ChildActorComponent|GetChildActor (Variables|Default|GetLine1WashLED1)))) (.AsBP%20Wash%20LEDCXZ (Utilities|Casting|CastToBP_WashLEDCXZ (Variables|/Script/Engine.ChildActorComponent|GetChildActor (Variables|Default|GetLine1WashLED7)))) (.AsBP%20Wash%20LEDCXZ (Utilities|Casting|CastToBP_WashLEDCXZ (Variables|/Script/Engine.ChildActorComponent|GetChildActor (Variables|Default|GetLine1WashLED3)))) (.AsBP%20Wash%20LEDCXZ (Utilities|Casting|CastToBP_WashLEDCXZ (Variables|/Script/Engine.ChildActorComponent|GetChildActor (Variables|Default|GetLine1WashLED4)))) (.AsBP%20Wash%20LEDCXZ (Utilities|Casting|CastToBP_WashLEDCXZ (Variables|/Script/Engine.ChildActorComponent|GetChildActor (Variables|Default|GetLine1WashLED6)))) (.AsBP%20Wash%20LEDCXZ (Utilities|Casting|CastToBP_WashLEDCXZ (Variables|/Script/Engine.ChildActorComponent|GetChildActor (Variables|Default|GetLine1WashLED5))))))
      (Variables|Default|SetMovingHeadsL2 (Utilities|Array|MakeArray (.AsBP%20Moving%20Head%20CXZ (Utilities|Casting|CastToBP_MovingHeadCXZ (Variables|/Script/Engine.ChildActorComponent|GetChildActor (Variables|Default|GetLine2MovingHead9)))) (.AsBP%20Moving%20Head%20CXZ (Utilities|Casting|CastToBP_MovingHeadCXZ (Variables|/Script/Engine.ChildActorComponent|GetChildActor (Variables|Default|GetLine2MovingHead2)))) (.AsBP%20Moving%20Head%20CXZ (Utilities|Casting|CastToBP_MovingHeadCXZ (Variables|/Script/Engine.ChildActorComponent|GetChildActor (Variables|Default|GetLine2MovingHead1)))) (.AsBP%20Moving%20Head%20CXZ (Utilities|Casting|CastToBP_MovingHeadCXZ (Variables|/Script/Engine.ChildActorComponent|GetChildActor (Variables|Default|GetLine2MovingHead4)))) (.AsBP%20Moving%20Head%20CXZ (Utilities|Casting|CastToBP_MovingHeadCXZ (Variables|/Script/Engine.ChildActorComponent|GetChildActor (Variables|Default|GetLine2MovingHead3)))) (.AsBP%20Moving%20Head%20CXZ (Utilities|Casting|CastToBP_MovingHeadCXZ (Variables|/Script/Engine.ChildActorComponent|GetChildActor (Variables|Default|GetLine2MovingHead8)))) (.AsBP%20Moving%20Head%20CXZ (Utilities|Casting|CastToBP_MovingHeadCXZ (Variables|/Script/Engine.ChildActorComponent|GetChildActor (Variables|Default|GetLine2MovingHead7)))) (.AsBP%20Moving%20Head%20CXZ (Utilities|Casting|CastToBP_MovingHeadCXZ (Variables|/Script/Engine.ChildActorComponent|GetChildActor (Variables|Default|GetLine2MovingHead6)))) (.AsBP%20Moving%20Head%20CXZ (Utilities|Casting|CastToBP_MovingHeadCXZ (Variables|/Script/Engine.ChildActorComponent|GetChildActor (Variables|Default|GetLine2MovingHead5)))))))
    (:then_1
      (for (_array_element _array_index) (Variables|Default|GetSM_TopLightLine1)
        (Rendering|Material|SetMaterial _array_element 0 (Variables|Default|GetMI_Light_Line1))
        (Transformation|SetRelativeLocation _array_element (Math|Vector|MakeVector 0.0 (* (- (Math|Conversions|ToFloat(Integer) _array_index) 3.5) 142.0) 0.0) false false))
      (for (_array_element_2 _array_index_2) (Variables|Default|GetSM_TopLightLine2)
        (Rendering|Material|SetMaterial _array_element_2 0 (Variables|Default|GetMI_Light_Line2))
        (Transformation|SetRelativeLocation _array_element_2 (Math|Vector|MakeVector 0.0 (* (- (Math|Conversions|ToFloat(Integer) _array_index_2) 3.5) 142.0) 0.0) false false))
      (for (_array_element_3 _array_index_3) (Variables|Default|GetWashLEDsL1)
        (Transformation|SetRelativeLocation (Class|Actor|GetParentComponent _array_element_3) (Math|Vector|MakeVector 0.0 (+ (* (- (Math|Conversions|ToFloat(Integer) _array_index_3) 3.5) 142.0) -71.0) 26.0) false false))
      (for (_array_element_4 _array_index_4) (Variables|Default|GetMovingHeadsL2)
        (Transformation|SetRelativeLocation (Class|Actor|GetParentComponent _array_element_4) (Math|Vector|MakeVector 0.0 (+ (* (- (Math|Conversions|ToFloat(Integer) _array_index_4) 3.5) 142.0) -71.0) 26.0) false false)))))