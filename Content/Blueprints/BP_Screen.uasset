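; Screen actor that cycles through images and videos loaded at runtime from the project's ScreenContent Pictures and Vedios folders.
; BeginPlay creates a media player, media texture and dynamic material on the screen mesh, then imports every picture as a texture.
; While Playing is set, CE_Next alternates between the full picture and video lists, swapping the material's texture parameter.
; Pictures hold for a fixed delay; videos poll until ready, then wait out their duration.
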(event Custom|CE_Next
  (if (not (and (== (Utilities|Array|Length (Variables|Default|GetPictures)) 0) (== (Utilities|Array|Length (Variables|Default|GetVedioFileNames)) 0)))
    (if (Variables|Default|GetPlaying)
      (if (Variables|Default|GetPlayingPictures)
        (Math|Integer|IncrementInt (Variables|Default|GetIdxPic)
          (:%20%20
            (if (Utilities|Array|IsValidIndex (Variables|Default|GetPictures) (Variables|Default|GetIdxPic))
              (CallFunction|CEPlayPicture (Utilities|Array|Get(acopy) (Variables|Default|GetPictures) (Variables|Default|GetIdxPic)))
              (else
                (Variables|Default|SetIdxPic -1)
                (Variables|Default|SetPlayingPictures false)
                (CallFunction|CENext)))))
        (else
          (Math|Integer|IncrementInt (Variables|Default|GetIdxVedio)
            (:%20%20
              (if (Utilities|Array|IsValidIndex (Variables|Default|GetVedioFileNames) (Variables|Default|GetIdxVedio))
                (CallFunction|CEPlayVedio (Utilities|String|Append (Utilities|String|Append (Class|BlueprintPathsLibrary|ProjectDir) "ScreenContent/Vedios/") (Utilities|Array|Get(acopy) (Variables|Default|GetVedioFileNames) (Variables|Default|GetIdxVedio))))
                (else
                  (Variables|Default|SetIdxVedio -1)
                  (Variables|Default|SetPlayingPictures true)
                  (CallFunction|CENext))))))))))

(event Custom|CE_PlayPicture
  (params (Pic :type Texture%20Object%20Reference))
  (Rendering|Material|SetTextureParameterValue (Variables|Default|GetMI) "Texture" Pic)
  (Utilities|FlowControl|Delay 5.0)
  (CallFunction|CENext))

(event Custom|CE_PlayVedio
  (params (FilePath :type String))
  (bind _mp (Variables|Default|GetMP))
  (Class|MediaPlayer|OpenFile (Variables|Default|GetMP) FilePath)
  (Rendering|Material|SetTextureParameterValue (Variables|Default|GetMI) "Texture" (Variables|Default|GetMT))
  (Media|MediaPlayer|Play _mp :!class /Script/MediaAssets.MediaPlayer)
  (if (Class|MediaPlayer|IsReady _mp) :!label _label
    (Utilities|FlowControl|Delay (Math|Timespan|GetTotalSeconds (Media|MediaPlayer|GetDuration _mp)))
    (CallFunction|CENext)
    (else
      (Utilities|FlowControl|Delay 0.05)
      (goto _label))))

(event EventBeginPlay
  (Utilities|FlowControl|Sequence
    (:then_0
      (CallFunction|FuncInitMediaPlayer)
      (bind _files (Class|CXZFuncLib|CXZGetFilenamesfromDir (Utilities|String|Append (Class|BlueprintPathsLibrary|ProjectDir) "ScreenContent/Pictures/") "*.*"))
      (Variables|Default|SetPictureFileNames _files)
      (bind _files_2 (Class|CXZFuncLib|CXZGetFilenamesfromDir (Utilities|String|Append (Class|BlueprintPathsLibrary|ProjectDir) "ScreenContent/Vedios/") "*.*"))
      (Variables|Default|SetVedioFileNames _files_2)
      (for _array_element (Variables|Default|GetPictureFileNames)
        (bind _returnvalue (Class|KismetRenderingLibrary|ImportFileasTexture2D (Utilities|String|Append (Utilities|String|Append (Class|BlueprintPathsLibrary|ProjectDir) "ScreenContent/Pictures/") _array_element)))
        (Utilities|Array|Add (Variables|Default|GetPictures) _returnvalue)))
    (:then_1
      (CallFunction|CENext))))

(fn ConstructionScript)

(fn FuncInitMediaPlayer
  (bind _returnvalue (Class|CXZFuncLib|CXZCreateMediaTexture))
  (Variables|Default|SetMT _returnvalue)
  (bind _returnvalue_2 (Game|ConstructObjectfromClass self "/Script/MediaAssets.MediaPlayer"))
  (Variables|Default|SetMP _returnvalue_2)
  (Media|MediaSoundComponent|SetMediaPlayer (Variables|Default|GetMT) (Variables|Default|GetMP))
  (bind _returnvalue_3 (Rendering|Material|CreateDynamicMaterialInstance (Variables|Default|GetSM_Screen) 0 "/Game/MyProject/Actors/Screen/M_Screen.M_Screen" "None" :!class /Script/Engine.PrimitiveComponent))
  (bind _output_get (Variables|Default|SetMI _returnvalue_3))
  (Rendering|Material|SetTextureParameterValue _output_get "Texture" (Variables|Default|GetMT)))