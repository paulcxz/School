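; BP_LectureHallPL is a switchable point light for a lecture hall, paired with a glowing sphere mesh.
; The construction script creates a dynamic instance of M_Light on the sphere and applies the configurable intensity and attenuation radius to the light.
; Custom events CE_TurnOn and CE_TurnOff set the light intensity and the material's Intensity parameter together, so the bulb's appearance follows the light state.
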(event Custom|CE_TurnOff
  (Rendering|Components|Light|SetIntensity (Variables|Default|GetPointLight) 0.0)
  (Rendering|Material|SetScalarParameterValue (Variables|Default|GetMI_Light) "Intensity" 0.0 :!class /Script/Engine.MaterialInstanceDynamic))

(event Custom|CE_TurnOn
  (Rendering|Components|Light|SetIntensity (Variables|Default|GetPointLight) (Variables|Default|GetIntensity))
  (Rendering|Material|SetScalarParameterValue (Variables|Default|GetMI_Light) "Intensity" 15.0 :!class /Script/Engine.MaterialInstanceDynamic))

(event EventBeginPlay)

(event Collision|EventActorBeginOverlap
  (params (OtherActor :type Actor%20Object%20Reference)))

(event EventTick
  (params (DeltaSeconds :type Float%20%28single-precision%29)))

(fn ConstructionScript
  (bind _returnvalue (Rendering|Material|CreateDynamicMaterialInstance (Variables|Default|GetSphere) 0 "/Game/Materials/M_Light.M_Light" "None" :!class /Script/Engine.PrimitiveComponent))
  (Variables|Default|SetMI_Light _returnvalue)
  (Rendering|Components|Light|SetIntensity (Variables|Default|GetPointLight) (Variables|Default|GetIntensity))
  (Rendering|Lighting|SetAttenuationRadius (Variables|Default|GetPointLight) (Variables|Default|GetAttenuation)))