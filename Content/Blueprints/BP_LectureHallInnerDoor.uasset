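; Lecture hall inner door whose left leaf swings in 90-degree yaw steps when the player's hand action hits either of its two handles.
; The sign of the stored angle and the OpenDir flag select a positive or negative timeline, while a moving flag blocks retriggering.
; Timeline handlers are written to rotate the door root, then update the angle and clear the flag.
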(event EventIPlayerHandAction
  (params (Hand :type EHand%20Enum :default "VR_LeftHand") (Comp :type Actor%20Component%20Object%20Reference))
  (if (or (== Comp (Variables|Default|GetLeftDoorHandle)) (== Comp (Variables|Default|GetLeftDoorHandle1)))
    (if (>= (Variables|Default|GetLeftDoorCurrentDegree) 0.0)
      (if (not (Variables|Default|GetLeftDoorMoving))
        (Variables|Default|SetLeftDoorMoving true)
        (Components|Timeline|PlayfromStart (select (Variables|Default|GetOpenDir) (Variables|Default|GetTL_LeftDoorTurnPos) (Variables|Default|GetTL_LeftDoorTurnNeg))))
      (elif (not (Variables|Default|GetLeftDoorMoving))
        (Variables|Default|SetLeftDoorMoving true)
        (Components|Timeline|PlayfromStart (select (Variables|Default|GetOpenDir) (Variables|Default|GetTL_LeftDoorTurnNeg) (Variables|Default|GetTL_LeftDoorTurnPos)))))))

(fn ConstructionScript)