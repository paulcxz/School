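; BP_Window is a parametric two-pane window with an outer frame, with no runtime logic.
; The construction script offsets the left and right sash roots in depth and width, then sizes each sash's glass and four bars from size, thickness and gap variables.
; It then fits the outer frame around both, deriving the sides from the top piece and a sash bar.
; Dimensions become world scales by dividing by 100.
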(event EventBeginPlay)

(event Collision|EventActorBeginOverlap
  (params (OtherActor :type Actor%20Object%20Reference)))

(event EventTick
  (params (DeltaSeconds :type Float%20%28single-precision%29)))

(fn ConstructionScript
  (bind _framet (Variables|Default|GetFrameT))
  (bind _framet_2 (Variables|Default|GetFrameT))
  (bind _windowframewidth (Variables|Default|GetWindowFrameWidth))
  (bind _windowframewidth_2 (Variables|Default|GetWindowFrameWidth))
  (bind _onewindowsize (Variables|Default|GetOneWindowSize))
  (bind _windowframewidth_3 (Variables|Default|GetWindowFrameWidth))
  (bind _leftwindowbarr (Variables|Default|GetLeftWindowBarR))
  (bind _onewindowsize_2 (Variables|Default|GetOneWindowSize))
  (bind _leftwindowbart (Variables|Default|GetLeftWindowBarT))
  (bind _onewindowsize_3 (Variables|Default|GetOneWindowSize))
  (bind _rightwindowbarr (Variables|Default|GetRightWindowBarR))
  (bind _onewindowsize_4 (Variables|Default|GetOneWindowSize))
  (bind _windowframewidth_4 (Variables|Default|GetWindowFrameWidth))
  (bind _windowframewidth_5 (Variables|Default|GetWindowFrameWidth))
  (bind _onewindowsize_5 (Variables|Default|GetOneWindowSize))
  (bind _windowframewidth_6 (Variables|Default|GetWindowFrameWidth))
  (bind _rightwindowbarl (Variables|Default|GetRightWindowBarL))
  (bind _rightwindowbart (Variables|Default|GetRightWindowBarT))
  (bind _windowframewidth_7 (Variables|Default|GetWindowFrameWidth))
  (bind _onewindowsize_6 (Variables|Default|GetOneWindowSize))
  (bind _windowframethickness (Variables|Default|GetWindowFrameThickness))
  (bind _windowframewidth_8 (Variables|Default|GetWindowFrameWidth))
  (bind _leftwindowbarl (Variables|Default|GetLeftWindowBarL))
  (bind _gapbetweenwindows (Variables|Default|GetGapBetweenWindows))
  (bind _framethickness (Variables|Default|GetFrameThickness))
  (bind _framethickness_2 (Variables|Default|GetFrameThickness))
  (bind _windowframewidth_9 (Variables|Default|GetWindowFrameWidth))
  (bind _framethickness_3 (Variables|Default|GetFrameThickness))
  (bind _windowframethickness_2 (Variables|Default|GetWindowFrameThickness))
  (bind _gapbetweenwindows_2 (Variables|Default|GetGapBetweenWindows))
  (bind _onewindowsize_7 (Variables|Default|GetOneWindowSize))
  (bind _gapbetweenwindows_3 (Variables|Default|GetGapBetweenWindows))
  (bind _returnvalue (Transformation|GetWorldScale _framet))
  (bind _returnvalue_2 (/ _windowframewidth_2 2.0))
  (bind _returnvalue_3 (Utilities|Operators|Subtract (.x _onewindowsize) _windowframewidth_3 _windowframewidth_3))
  (bind _returnvalue_4 (- (.x _onewindowsize_2) _windowframewidth))
  (bind _returnvalue_5 (- (.y _onewindowsize_3) _windowframewidth_7))
  (bind _returnvalue_6 (- (.x _onewindowsize_4) _windowframewidth_4))
  (bind _returnvalue_7 (/ _windowframewidth_5 2.0))
  (bind _returnvalue_8 (Utilities|Operators|Subtract (.x _onewindowsize_5) _windowframewidth_6 _windowframewidth_6))
  (bind _returnvalue_9 (- (.y _onewindowsize_6) _windowframewidth_8))
  (bind _returnvalue_10 (/ _windowframethickness_2 2.0))
  (bind _returnvalue_11 (* _gapbetweenwindows 3.0))
  (bind _returnvalue_12 (* _framethickness_2 2.0))
  (bind _returnvalue_13 (* _windowframethickness 2.0))
  (bind _returnvalue_14 (/ (.y _onewindowsize_7) 2.0))
  (bind _returnvalue_15 (/ _framethickness 2.0))
  (bind _relativelocation (Variables|/Script/Engine.SceneComponent|GetRelativeLocation _framet_2))
  (bind _returnvalue_16 (* (.y _returnvalue) 5e+01))
  (bind _returnvalue_17 (/ _returnvalue_3 2.0))
  (bind _returnvalue_18 (/ _returnvalue_4 1e+02))
  (bind _returnvalue_19 (/ _returnvalue_5 2.0))
  (bind _returnvalue_20 (/ _returnvalue_6 1e+02))
  (bind _returnvalue_21 (/ _returnvalue_8 2.0))
  (bind _returnvalue_22 (/ _returnvalue_9 2.0))
  (bind _returnvalue_23 (+ _returnvalue_10 _gapbetweenwindows_2 _framethickness_3))
  (bind _returnvalue_24 (+ _returnvalue_12 _returnvalue_13 _returnvalue_11))
  (bind _returnvalue_25 (+ _returnvalue_14 _returnvalue_15 _gapbetweenwindows_3))
  (bind _returnvalue_26 (+ _returnvalue_17 _returnvalue_2))
  (bind _returnvalue_27 (+ _returnvalue_21 _returnvalue_7))
  (bind _returnvalue_28 (/ _returnvalue_24 2.0))
  (bind _returnvalue_29 (* _returnvalue_26 -1.0))
  (bind _returnvalue_30 (* _returnvalue_27 -1.0))
  (bind _returnvalue_31 (- _returnvalue_23 _returnvalue_28))
  (bind _returnvalue_32 (* _returnvalue_31 -1.0))
  (Utilities|FlowControl|Sequence
    (:then_0
      (bind _output_get (Variables|Default|SetWindowOriYPosR (.x (Variables|Default|GetOneWindowSize))))
      (Transformation|SetRelativeLocation (Variables|Default|GetRootRightWindow) (Math|Vector|MakeVector 0.0 _output_get 0.0) false false)
      (Variables|Default|SetWindowOriYPosL (Variables|Default|GetWindowFrameWidth))
      (Transformation|SetRelativeLocation (Variables|Default|GetRootLeftWindow) (Math|Vector|MakeVector (+ (Variables|Default|GetWindowFrameThickness) (Variables|Default|GetGapBetweenWindows)) (Variables|Default|GetWindowOriYPosL) 0.0) false false))
    (:then_1
      (Transformation|SetRelativeLocation (Variables|Default|GetRightWindowGlass) (Math|Vector|MakeVector 0.0 _returnvalue_30 0.0) false false)
      (Transformation|SetWorldScale3D (Variables|Default|GetRightWindowGlass) (Math|Vector|MakeVector (/ (Variables|Default|GetGlassThickness) 1e+02) _returnvalue_20 (/ (- (.y _onewindowsize_4) _windowframewidth_4) 1e+02)))
      (Transformation|SetWorldScale3D _rightwindowbarr (Math|Vector|MakeVector (/ (Variables|Default|GetWindowFrameThickness) 1e+02) (/ (Variables|Default|GetWindowFrameWidth) 1e+02) (/ (.y (Variables|Default|GetOneWindowSize)) 1e+02)))
      (Transformation|SetRelativeLocation _rightwindowbarr (Math|Vector|MakeVector 0.0 0.0 0.0) false false)
      (Transformation|SetWorldScale3D _rightwindowbarl (Math|Vector|MakeVector (/ (Variables|Default|GetWindowFrameThickness) 1e+02) (/ (Variables|Default|GetWindowFrameWidth) 1e+02) (/ (.y (Variables|Default|GetOneWindowSize)) 1e+02)))
      (Transformation|SetRelativeLocation _rightwindowbarl (Math|Vector|MakeVector 0.0 (* _returnvalue_27 -2.0) 0.0) false false)
      (Transformation|SetWorldScale3D _rightwindowbart (Math|Vector|MakeVector (/ (Variables|Default|GetWindowFrameThickness) 1e+02) _returnvalue_20 (/ (Variables|Default|GetWindowFrameWidth) 1e+02)))
      (Transformation|SetRelativeLocation _rightwindowbart (Math|Vector|MakeVector 0.0 _returnvalue_30 _returnvalue_22) false false)
      (Transformation|SetRelativeLocation (Variables|Default|GetRightWindowBarB) (Math|Vector|MakeVector 0.0 _returnvalue_30 (* _returnvalue_22 -1.0)) false false))
    (:then_2
      (Transformation|SetRelativeLocation (Variables|Default|GetLeftWindowGlass) (Math|Vector|MakeVector 0.0 _returnvalue_29 0.0) false false)
      (Transformation|SetWorldScale3D (Variables|Default|GetLeftWindowGlass) (Math|Vector|MakeVector (/ (Variables|Default|GetGlassThickness) 1e+02) _returnvalue_18 (/ (- (.y _onewindowsize_2) _windowframewidth) 1e+02)))
      (Transformation|SetWorldScale3D _leftwindowbarr (Math|Vector|MakeVector (/ (Variables|Default|GetWindowFrameThickness) 1e+02) (/ (Variables|Default|GetWindowFrameWidth) 1e+02) (/ (.y (Variables|Default|GetOneWindowSize)) 1e+02)))
      (Transformation|SetRelativeLocation _leftwindowbarr (Math|Vector|MakeVector 0.0 0.0 0.0) false false)
      (Transformation|SetWorldScale3D _leftwindowbarl (Math|Vector|MakeVector (/ (Variables|Default|GetWindowFrameThickness) 1e+02) (/ (Variables|Default|GetWindowFrameWidth) 1e+02) (/ (.y (Variables|Default|GetOneWindowSize)) 1e+02)))
      (Transformation|SetRelativeLocation _leftwindowbarl (Math|Vector|MakeVector 0.0 (* _returnvalue_26 -2.0) 0.0) false false)
      (Transformation|SetWorldScale3D _leftwindowbart (Math|Vector|MakeVector (/ (Variables|Default|GetWindowFrameThickness) 1e+02) _returnvalue_18 (/ (Variables|Default|GetWindowFrameWidth) 1e+02)))
      (Transformation|SetRelativeLocation _leftwindowbart (Math|Vector|MakeVector 0.0 _returnvalue_29 _returnvalue_19) false false)
      (Transformation|SetRelativeLocation (Variables|Default|GetLeftWindowBarB) (Math|Vector|MakeVector 0.0 _returnvalue_29 (* _returnvalue_19 -1.0)) false false))
    (:then_3
      (Transformation|SetWorldScale3D (Variables|Default|GetFrameB) (Math|Vector|MakeVector (/ (+ (* (Variables|Default|GetWindowFrameThickness) 2.0) (* (Variables|Default|GetGapBetweenWindows) 3.0)) 1e+02) (/ (+ (- (* (.x (Variables|Default|GetOneWindowSize)) 2.0) (Variables|Default|GetWindowFrameWidth)) (* (Variables|Default|GetFrameThickness) 2.0)) 1e+02) (/ (Variables|Default|GetFrameThickness) 1e+02)))
      (Transformation|SetRelativeLocation (Variables|Default|GetFrameB) (Math|Vector|MakeVector _returnvalue_32 _windowframewidth_9 (* _returnvalue_25 -1.0)) false false)
      (Transformation|SetRelativeLocation (Variables|Default|GetFrameT) (Math|Vector|MakeVector _returnvalue_32 _windowframewidth_9 _returnvalue_25) false false)
      (Transformation|SetWorldScale3D (Variables|Default|GetFrameL) (Math|Vector|MakeVector (.x (Transformation|GetWorldScale (Variables|Default|GetFrameT))) (/ (Variables|Default|GetFrameThickness) 1e+02) (/ (+ (* (.z (Transformation|GetWorldScale (Variables|Default|GetLeftWindowBarL))) 1e+02) (* (Variables|Default|GetGapBetweenWindows) 2.0) (* (Variables|Default|GetFrameThickness) 2.0)) 1e+02)))
      (Transformation|SetRelativeLocation (Variables|Default|GetFrameR) (Math|Vector|MakeVector (.x _relativelocation) (- (.y _relativelocation) _returnvalue_16) 0.0) false false)
      (Transformation|SetRelativeLocation (Variables|Default|GetFrameL) (Math|Vector|MakeVector (.x _relativelocation) (+ (.y _relativelocation) _returnvalue_16) 0.0) false false))))