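; BP_Chair is a chair actor that sets which of its two handles are visible.
; Func_InitHandle always shows RootHandleR and shows RootHandleL only when the actor has the "LastOne" tag or HasRightHandle is true, propagating visibility to children.
; It runs from both the Construction Script and BeginPlay, so the handle setup applies at construction and again when play starts.
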(event EventBeginPlay
  (CallFunction|FuncInitHandle))

(event Collision|EventActorBeginOverlap
  (params (OtherActor :type Actor%20Object%20Reference)))

(event EventTick
  (params (DeltaSeconds :type Float%20%28single-precision%29)))

(fn ConstructionScript
  (CallFunction|FuncInitHandle))

(fn FuncInitHandle
  (bind _roothandler (Variables|Default|GetRootHandleR))
  (bind _roothandlel (Variables|Default|GetRootHandleL))
  (if (or (Actor|ActorHasTag "LastOne") (Variables|Default|GetHasRightHandle))
    (Rendering|SetVisibility _roothandler true true)
    (Rendering|SetVisibility _roothandlel true true)
    (else
      (Rendering|SetVisibility _roothandler true true)
      (Rendering|SetVisibility _roothandlel false true))))