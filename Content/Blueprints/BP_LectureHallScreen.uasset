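; Lecture hall screen actor that plays a video file with sound on its screen mesh.
; On BeginPlay it builds a media player and media texture at runtime, binding them to a dynamic screen material and the media sound component at a set volume.
; After a short delay, a custom event opens and plays a video from a hard-coded absolute D: drive path; the project-relative path logic is unused.
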(event Custom|CE_PlayVedio
  (params (FilePath :type String))
  (Class|MediaPlayer|OpenFile (Variables|Default|GetMP) FilePath)
  (Media|MediaPlayer|Play (Variables|Default|GetMP) :!class /Script/MediaAssets.MediaPlayer))

(event EventBeginPlay
  (CallFunction|FuncInitMediaPlayer)
  (Utilities|FlowControl|Delay 0.2)
  (CallFunction|CEPlayVedio "D:/电子屏素材/国测/视频/《迎接亚运会》.mp4"))

(event Collision|EventActorBeginOverlap
  (params (OtherActor :type Actor%20Object%20Reference)))

(event EventTick
  (params (DeltaSeconds :type Float%20%28single-precision%29)))

(fn ConstructionScript)

(fn FuncInitMediaPlayer
  (bind _returnvalue (Class|CXZFuncLib|CXZCreateMediaTexture))
  (Variables|Default|SetMT _returnvalue)
  (bind _returnvalue_2 (Game|ConstructObjectfromClass self "/Script/MediaAssets.MediaPlayer"))
  (bind _output_get (Variables|Default|SetMP _returnvalue_2))
  (Media|MediaSoundComponent|SetMediaPlayer (Variables|Default|GetMT) _output_get)
  (bind _returnvalue_3 (Rendering|Material|CreateDynamicMaterialInstance (Variables|Default|GetSM_Screen) 1 "/Game/MyProject/Actors/Screen/M_Screen.M_Screen" "None" :!class /Script/Engine.PrimitiveComponent))
  (bind _output_get_2 (Variables|Default|SetMI _returnvalue_3))
  (Rendering|Material|SetTextureParameterValue _output_get_2 "Texture" (Variables|Default|GetMT))
  (Media|MediaSoundComponent|SetMediaPlayer (Variables|Default|GetMediaSound) (Variables|Default|GetMP))
  (Audio|Components|Audio|SetVolumeMultiplier (Variables|Default|GetMediaSound) (Variables|Default|GetVolume) :!class /Script/AudioMixer.SynthComponent))