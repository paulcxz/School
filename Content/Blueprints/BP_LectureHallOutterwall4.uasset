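; Lecture hall outer wall with a double door that the player opens and closes by hand through two handles on each leaf.
; The player hand interface event picks a timeline from the handle used and that door's current angle, so a closed door swings in opposite directions per handle and an open one swings back.
; Timelines rotate each door root a quarter turn, then store the new angle, with per-door moving flags blocking overlapping swings.
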(event EventIPlayerHandAction
  (params (Hand :type EControllerHand%20Enum :default "Left") (Comp :type Actor%20Component%20Object%20Reference))
  (if (== Comp (Variables|Default|GetLeftDoorHandle))
    (if (>= (Variables|Default|GetLeftDoorCurrentDegree) 0.0)
      (if (not (Variables|Default|GetLeftDoorMoving)) :!label _label
        (Variables|Default|SetLeftDoorMoving true)
        (Components|Timeline|PlayfromStart (Variables|Default|GetTL_LeftDoorTurnNeg)))
      (else
        (if (not (Variables|Default|GetLeftDoorMoving)) :!label _label_2
          (Variables|Default|SetLeftDoorMoving true)
          (Components|Timeline|PlayfromStart (Variables|Default|GetTL_LeftDoorTurnPos)))))
    (elif (== Comp (Variables|Default|GetLeftDoorHandle1))
      (if (<= (Variables|Default|GetLeftDoorCurrentDegree) 0.0)
        (goto _label_2)
        (else
          (goto _label)))
      (elif (== Comp (Variables|Default|GetRightDoorHandle))
        (if (<= (Variables|Default|GetRightDoorCurrentDegree) 0.0)
          (if (not (Variables|Default|GetRightDoorMoving)) :!label _label_3
            (Variables|Default|SetRightDoorMoving true)
            (Components|Timeline|PlayfromStart (Variables|Default|GetTL_RightDoorTurnPos)))
          (else
            (if (not (Variables|Default|GetRightDoorMoving)) :!label _label_4
              (Variables|Default|SetRightDoorMoving true)
              (Components|Timeline|PlayfromStart (Variables|Default|GetTL_RightDoorTurnNeg)))))
        (elif (== Comp (Variables|Default|GetRightDoorHandle1))
          (if (>= (Variables|Default|GetRightDoorCurrentDegree) 0.0)
            (goto _label_4)
            (else
              (goto _label_3))))))))

(fn ConstructionScript)