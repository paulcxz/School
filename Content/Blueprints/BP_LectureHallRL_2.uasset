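; BP_LectureHallRL_2 is a lecture hall light fixture that pairs a rect light with a row of fourteen production-light meshes.
; The construction script spaces the meshes evenly along Y, centered on the origin, and gives them one shared dynamic emissive material instance.
; CE_TurnOn and CE_TurnOff switch the rect light intensity and that material's Intensity parameter together, so the whole row lights or darkens at once.
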(event Custom|CE_TurnOff
  (Rendering|Components|Light|SetIntensity (Variables|Default|GetRectLight) 0.0)
  (Rendering|Material|SetScalarParameterValue (Variables|Default|GetMI_Light) "Intensity" 0.0 :!class /Script/Engine.MaterialInstanceDynamic))

(event Custom|CE_TurnOn
  (Rendering|Components|Light|SetIntensity (Variables|Default|GetRectLight) (Variables|Default|GetIntensity))
  (Rendering|Material|SetScalarParameterValue (Variables|Default|GetMI_Light) "Intensity" 15.0 :!class /Script/Engine.MaterialInstanceDynamic))

(event EventBeginPlay)

(event Collision|EventActorBeginOverlap
  (params (OtherActor :type Actor%20Object%20Reference)))

(event EventTick
  (params (DeltaSeconds :type Float%20%28single-precision%29)))

(fn ConstructionScript
  (Variables|Default|SetSM_Lights (Utilities|Array|MakeArray (Variables|Default|GetSM_Production_Light_01c4) (Variables|Default|GetSM_Production_Light_01c3) (Variables|Default|GetSM_Production_Light_01c2) (Variables|Default|GetSM_Production_Light_01c1) (Variables|Default|GetSM_Production_Light_01c) (Variables|Default|GetSM_Production_Light_01c5) (Variables|Default|GetSM_Production_Light_01c13) (Variables|Default|GetSM_Production_Light_01c12) (Variables|Default|GetSM_Production_Light_01c11) (Variables|Default|GetSM_Production_Light_01c10) (Variables|Default|GetSM_Production_Light_01c9) (Variables|Default|GetSM_Production_Light_01c8) (Variables|Default|GetSM_Production_Light_01c7) (Variables|Default|GetSM_Production_Light_01c6)))
  (bind _returnvalue (Rendering|Material|CreateDynamicMaterialInstance "/Game/Hollywood_Vol3/Materials/Instances/MI_Stage_Lights_01a.MI_Stage_Lights_01a" "None" "None" :!class /Script/Engine.KismetMaterialLibrary))
  (bind _output_get (Variables|Default|SetMI_Light _returnvalue))
  (Rendering|Material|SetVectorParameterValue _output_get "Emissive Color Multi" "(R=10.000000,G=10.000000,B=10.000000,A=1.000000)" :!class /Script/Engine.MaterialInstanceDynamic)
  (for (_array_element _array_index) (Variables|Default|GetSM_Lights)
    (Rendering|Material|SetMaterial _array_element 0 (Variables|Default|GetMI_Light))
    (Transformation|SetRelativeLocation _array_element (Math|Vector|MakeVector 0.0 (* (- (Math|Conversions|ToFloat(Integer) _array_index) 6.5) 1e+02) 15.0) false false)))