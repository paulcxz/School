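; BP_LectureHallF2DoorPlacer1 is an actor Blueprint, named as a door placer for a lecture hall's second floor, that can clear walls.
; Func_ClearWalls runs four sequential loops over arrays, destroying the child actor held by each element.
; The event graph and construction script are empty, so nothing in this Blueprint calls the function or places doors.
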(event EventBeginPlay)

(event Collision|EventActorBeginOverlap
  (params (OtherActor :type Actor%20Object%20Reference)))

(event EventTick
  (params (DeltaSeconds :type Float%20%28single-precision%29)))

(fn ConstructionScript)

(fn FuncClearWalls
  (for _array_element 0
    (Actor|DestroyActor (Variables|/Script/Engine.ChildActorComponent|GetChildActor _array_element)))
  (for _array_element_2 0
    (Actor|DestroyActor (Variables|/Script/Engine.ChildActorComponent|GetChildActor _array_element_2)))
  (for _array_element_3 0
    (Actor|DestroyActor (Variables|/Script/Engine.ChildActorComponent|GetChildActor _array_element_3)))
  (for _array_element_4 0
    (Actor|DestroyActor (Variables|/Script/Engine.ChildActorComponent|GetChildActor _array_element_4))))