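; Builder actor that assembles the curved walls and gate walls of a lecture hall on two floors.
; The construction script clears previous walls, then spawns child actor components in loops, stepping yaw around the actor's origin to form a ring of walls with a gate section.
; F1 pieces repeat the F2 layout at lowered heights, and each group is stored in its own array for cleanup.
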(event EventBeginPlay)

(event Collision|EventActorBeginOverlap
  (params (OtherActor :type Actor%20Object%20Reference)))

(event EventTick
  (params (DeltaSeconds :type Float%20%28single-precision%29)))

(fn ConstructionScript
  (CallFunction|FuncClearWalls)
  (Utilities|FlowControl|Sequence
    (:then_0
      (for _index (range 0 108)
        (bind _returnvalue (AddComponent|AddChildActorComponent false (Math|Transform|MakeTransform "0, 0, 0" (Math|Rotator|MakeRotator 0.0 0.0 (+ -1e+01 (* _index -3.135))) "1.000000,1.000000,1.000000")))
        (Utilities|Array|Add (Variables|Default|GetWallsF2) _returnvalue)))
    (:then_1
      (for _index_2 (range 0 2)
        (bind _returnvalue_2 (AddComponent|AddChildActorComponent false (Math|Transform|MakeTransform "0, 0, 0" (Math|Rotator|MakeRotator 0.0 0.0 (+ 6.9 (* _index_2 -6.05))) "1.000000,1.000000,1.000000")))
        (Utilities|Array|Add (Variables|Default|GetGateWallsF2) _returnvalue_2)))
    (:then_2
      (for _index_3 (range 0 108)
        (bind _returnvalue_3 (AddComponent|AddChildActorComponent false (Math|Transform|MakeTransform "0, 0,-730.000000" (Math|Rotator|MakeRotator 0.0 0.0 (+ -1e+01 (* _index_3 -3.135))) "1.000000,1.000000,1.000000")))
        (Utilities|Array|Add (Variables|Default|GetWallsF1) _returnvalue_3)))
    (:then_3
      (for _index_4 (range 0 2)
        (bind _returnvalue_4 (AddComponent|AddChildActorComponent false (Math|Transform|MakeTransform "0, 0,-515.000000" (Math|Rotator|MakeRotator 0.0 0.0 (+ 6.75 (* _index_4 -6.05))) "1.000000,1.000000,1.000000")))
        (Utilities|Array|Add (Variables|Default|GetGateWallsF1) _returnvalue_4)))))

(fn FuncClearWalls
  (for _array_element (Variables|Default|GetWallsF2)
    (Actor|DestroyActor (Variables|/Script/Engine.ChildActorComponent|GetChildActor _array_element)))
  (for _array_element_2 (Variables|Default|GetGateWallsF2)
    (Actor|DestroyActor (Variables|/Script/Engine.ChildActorComponent|GetChildActor _array_element_2)))
  (for _array_element_3 (Variables|Default|GetWallsF1)
    (Actor|DestroyActor (Variables|/Script/Engine.ChildActorComponent|GetChildActor _array_element_3)))
  (for _array_element_4 (Variables|Default|GetGateWallsF1)
    (Actor|DestroyActor (Variables|/Script/Engine.ChildActorComponent|GetChildActor _array_element_4))))