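; BP_Curtain is a curtain actor with a skeletal mesh, a configurable material and an optional visible track.
; Construction applies the material and sets track visibility.
; On BeginPlay it casts the mesh's anim instance to ABP_Curtain and passes it the Min and Max limits.
; Timeline logic to drive the anim Percent and cloth blend weight exists but is disconnected, so the graph never animates the curtain.
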(event EventBeginPlay
  (bind _asabp_curtain (Utilities|Casting|CastToABP_Curtain (Components|SkeletalMesh|GetAnimInstance (Variables|Default|GetSkeletalMesh))))
  (bind _output_get (Variables|Default|SetAniInstCurtain _asabp_curtain))
  (Variables|/Game/MyProject/Actors/Curtain/ABP_Curtain.ABP_Curtain_C|SetMin _output_get (Variables|Default|GetMin))
  (Variables|/Game/MyProject/Actors/Curtain/ABP_Curtain.ABP_Curtain_C|SetMax _output_get (Variables|Default|GetMax)))

(event Collision|EventActorBeginOverlap
  (params (OtherActor :type Actor%20Object%20Reference)))

(event EventTick
  (params (DeltaSeconds :type Float%20%28single-precision%29)))

(fn ConstructionScript
  (Rendering|Material|SetMaterial (Variables|Default|GetSkeletalMesh) 0 (Variables|Default|GetCurtainMat))
  (Rendering|SetVisibility (Variables|Default|GetCube) (Variables|Default|GetTrackVisable) false))