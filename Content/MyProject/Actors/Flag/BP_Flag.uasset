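; Flag actor for a flag-raising ceremony: CE_Raise plays the national anthem and Tick lifts the flag over the song's length.
; A WindDirectionalSource spawned and attached on BeginPlay follows randomized yaw, strength and speed targets from three looping delays, smoothed each Tick.
; After a fixed delay in the raise, the PlayerPawn shows the flag full screen and the wind locks to a strong fixed direction.
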(event Custom|CE_Raise
  (if (not (Variables|Default|GetRaising))
    (Variables|Default|SetRaising true)
    (Audio|PlaySound2D "/Game/国歌.国歌" 1.0 1.0 0.0 0 0)
    (Utilities|FlowControl|Delay 48.0)
    (bind _asplayer_pawn (Utilities|Casting|CastToPlayerPawn (Game|Player|GetPlayerPawn 0)))
    (Default|CEShowFlagFullScreen _asplayer_pawn)
    (Variables|Default|SetIsShowFullScreen true)))

(event EventTick
  (params (DeltaSeconds :type Float%20%28single-precision%29))
  (CallFunction|FuncUpdateFlagPos DeltaSeconds)
  (CallFunction|FuncUpdateWind DeltaSeconds))

(event EventBeginPlay
  (bind _returnvalue (Transformation|GetActorRotation))
  (bind _returnvalue_2 (Game|SpawnActorfromClass "/Script/Engine.WindDirectionalSource" (Math|Transform|MakeTransform "0, 0, 0" "0, 0, 0" "1,1,1") "AlwaysSpawn" 0 0))
  (bind _output_get (Variables|Default|SetWind _returnvalue_2))
  (Transformation|AttachActorToActor _output_get self "None" "SnapToTarget" "SnapToTarget" "KeepWorld" true)
  (Utilities|FlowControl|Sequence
    (:then_0
      (Variables|Default|SetTargetZR (Math|Random|RandomFloatinRange (- (.yaw _returnvalue) 45.0) (- (.yaw _returnvalue) -45.0)) :!label _label)
      (Utilities|FlowControl|Delay (Math|Random|RandomFloatinRange 0.2 1.8))
      (goto _label))
    (:then_1
      (Variables|Default|SetTargetStrength (Math|Random|RandomFloatinRange 0.8 2.0) :!label _label_2)
      (Utilities|FlowControl|Delay (Math|Random|RandomFloatinRange 2.0 4.0))
      (goto _label_2))
    (:then_2
      (Variables|Default|SetTargetSpeed (Math|Random|RandomFloatinRange 0.8 1.2) :!label _label_3)
      (Utilities|FlowControl|Delay (Math|Random|RandomFloatinRange 1.0 4.5))
      (goto _label_3))))

(event Collision|EventActorBeginOverlap
  (params (OtherActor :type Actor%20Object%20Reference)))

(fn ConstructionScript)

(fn FuncUpdateWind
  (params (DeltaTime :type Float%20%28single-precision%29))
  (bind _wind (Variables|Default|GetWind))
  (bind _wind_2 (Variables|Default|GetWind))
  (bind _component (Variables|/Script/Engine.WindDirectionalSource|GetComponent _wind))
  (bind _component_2 (Variables|/Script/Engine.WindDirectionalSource|GetComponent _wind_2))
  (if (Variables|Default|GetIsShowFullScreen)
    (Transformation|SetActorRotation (Variables|Default|GetWind) (Math|Rotator|MakeRotator 0.0 0.0 1.8e+02))
    (Class|WindDirectionalSourceComponent|SetStrength (Variables|/Script/Engine.WindDirectionalSource|GetComponent (Variables|Default|GetWind)) 4.0)
    (Class|WindDirectionalSourceComponent|SetSpeed (Variables|/Script/Engine.WindDirectionalSource|GetComponent (Variables|Default|GetWind)) 5.0)
    (else
      (Transformation|SetActorRotation (Variables|Default|GetWind) (Math|Rotator|MakeRotator 0.0 0.0 (.yaw (Math|Interpolation|RInterpTo (Transformation|GetActorRotation (Variables|Default|GetWind)) (Math|Rotator|MakeRotator 0.0 0.0 (Variables|Default|GetTargetZR)) DeltaTime 5.0))))
      (Class|WindDirectionalSourceComponent|SetStrength _component (Math|Interpolation|FInterpTo (Variables|/Script/Engine.WindDirectionalSourceComponent|GetStrength _component) (Variables|Default|GetTargetStrength) DeltaTime 6.0))
      (Class|WindDirectionalSourceComponent|SetSpeed _component_2 (Math|Interpolation|FInterpTo (Variables|/Script/Engine.WindDirectionalSourceComponent|GetSpeed _component_2) (Variables|Default|GetTargetSpeed) DeltaTime 4.0)))))

(fn FuncUpdateFlagPos
  (params (DeltaT :type Float%20%28single-precision%29))
  (if (Variables|Default|GetRaising)
    (bind _output_get (Variables|Default|SetTimeElapsed (+ (stale _output_get) DeltaT)))
    (Transformation|SetRelativeLocation (Variables|Default|Getflag) (Math|Vector|MakeVector 0.0 0.0 (Math|Float|MapRangeClamped (Variables|Default|GetTimeElapsed) 0.0 (Variables|Default|GetSongLength) -42.0 509.0)) false true)))