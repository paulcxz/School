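; BP_Xiaohui is a school emblem actor that lays out eleven components named for the syllables of "Wen Zhou Shang Hai Shi Jie Wai Guo Yu Xue Xiao" along a spline.
; The Construction Script derives an end margin from the Cylinder's world X scale and spaces the components evenly between both margins.
; Each takes the spline's local location and rotation at its distance, raised slightly in Z.
; The event graph is unused.
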(event EventBeginPlay)

(event Collision|EventActorBeginOverlap
  (params (OtherActor :type Actor%20Object%20Reference)))

(event EventTick
  (params (DeltaSeconds :type Float%20%28single-precision%29)))

(fn ConstructionScript
  (Variables|Default|SetHeadLength (* (.x (Transformation|GetWorldScale (Variables|Default|GetCylinder))) 33.0))
  (LocalVariables|Setl_SpaceEachChar (/ (- (Spline|GetSplineLength (Variables|Default|GetSpline)) (* (Variables|Default|GetHeadLength) 2.0)) 1e+01))
  (LocalVariables|Setl_CharArray (Utilities|Array|MakeArray (Variables|Default|Getwen) (Variables|Default|Getzhou) (Variables|Default|Getshang) (Variables|Default|Gethai) (Variables|Default|Getshi) (Variables|Default|Getjie) (Variables|Default|Getwai) (Variables|Default|Getguo) (Variables|Default|Getyu) (Variables|Default|Getxue) (Variables|Default|Getxiao)))
  (for _index (range 0 10)
    (LocalVariables|Setl_Idx _index)
    (Transformation|SetRelativeLocationAndRotation (Utilities|Array|Get(acopy) (LocalVariables|Getl_CharArray) (LocalVariables|Getl_Idx)) (+ (.Location (Math|Transform|BreakTransform (Spline|GetTransformatDistanceAlongSpline (Variables|Default|GetSpline) (+ (Variables|Default|GetHeadLength) (* (LocalVariables|Getl_Idx) (LocalVariables|Getl_SpaceEachChar))) "Local" true))) "0, 0,10.000000") (.Rotation (Math|Transform|BreakTransform (Spline|GetTransformatDistanceAlongSpline (Variables|Default|GetSpline) (+ (Variables|Default|GetHeadLength) (* (LocalVariables|Getl_Idx) (LocalVariables|Getl_SpaceEachChar))) "Local" true))) false false)))