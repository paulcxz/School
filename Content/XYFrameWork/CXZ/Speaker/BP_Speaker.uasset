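; BP_Speaker is a placeable speaker actor that plays a playlist of media files through a MediaSound component, with optional spatial attenuation.
; Init, run on construction and BeginPlay, applies the mesh, creates a MediaPlayer and MediaPlaylist if missing, and picks attenuation by falloff distance.
; The ExposedVariables map can override the attenuation flag.
; Interface events control play, stop, looping, volume and playlist replacement, which removes entries by ascending index before adding files.
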(event EventISetLooping
  (params (Looping :type Boolean))
  (Components|Timeline|SetLooping (Variables|Default|GetMediaPlayer) Looping))

(event EventIPlayAudio
  (Class|MediaPlayer|OpenPlaylist (Variables|Default|GetMediaPlayer) (Variables|Default|GetPlayList)))

(event EventIStopAudio
  (Media|MediaPlayer|Close (Variables|Default|GetMediaPlayer) :!class /Script/MediaAssets.MediaPlayer))

(event EventISetVolume
  (params (Volume :type Float%20%28double-precision%29))
  (Audio|Components|Audio|SetVolumeMultiplier (Variables|Default|GetMediaSound) Volume :!class /Script/AudioMixer.SynthComponent))

(event EventISetPlayList
  (params (List :type Array%20of%20Strings))
  (CallFunction|FuncSetPlayList List))

(event EventBeginPlay
  (CallFunction|Init))

(fn ConstructionScript
  (bind _exposedvariables (Variables|Default|GetExposedVariables))
  (bind (_value _returnvalue) (Utilities|Map|Find _exposedvariables "Attenuation"))
  (if _returnvalue
    (Variables|Default|SetAttenuation (Utilities|Enum|Equal(Enum) _value "true")))
  (CallFunction|Init))

(fn Init
  (Components|StaticMesh|SetStaticMesh (Variables|Default|GetStaticMesh) (Variables|Default|GetSpeakerMesh))
  (Transformation|SetWorldScale3D (Variables|Default|GetStaticMesh) (Variables|Default|GetSpeakerMeshScale))
  (Variables|/Script/AudioMixer.SynthComponent|SetbAllowSpatialization (Variables|Default|GetMediaSound) (Variables|Default|GetAttenuation))
  (Utilities|FlowControl|Sequence
    (:then_0
      (if (not (Utilities|IsValid (Variables|Default|GetMediaPlayer)))
        (bind _returnvalue (Game|ConstructObjectfromClass self "/Script/MediaAssets.MediaPlayer"))
        (bind _output_get (Variables|Default|SetMediaPlayer _returnvalue))
        (Media|MediaSoundComponent|SetMediaPlayer (Variables|Default|GetMediaSound) _output_get)
        (Audio|Components|Audio|SetVolumeMultiplier (Variables|Default|GetMediaSound) (Variables|Default|GetVolume) :!class /Script/AudioMixer.SynthComponent)
        (Variables|/Script/AudioMixer.SynthComponent|SetAttenuationSettings (Variables|Default|GetMediaSound) (Utilities|Select :Index (Variables|Default|GetFallOffDistance) :NewEnumerator0 "/Game/XYFrameWork/CXZ/Speaker/Attenuation_Speaker_F30.Attenuation_Speaker_F30" :NewEnumerator1 "/Game/XYFrameWork/CXZ/Speaker/Attenuation_Speaker_F60.Attenuation_Speaker_F60" :NewEnumerator2 "/Game/XYFrameWork/CXZ/Speaker/Attenuation_Speaker_F150.Attenuation_Speaker_F150"))))
    (:then_1
      (if (not (Utilities|IsValid (Variables|Default|GetPlayList)))
        (bind _returnvalue_2 (Game|ConstructObjectfromClass self "/Script/MediaAssets.MediaPlaylist"))
        (Variables|Default|SetPlayList _returnvalue_2)))))

(fn FuncSetPlayList
  (params (NewList :type Array%20of%20Strings))
  (Utilities|FlowControl|Sequence
    (:then_0
      (bind _returnvalue (Class|MediaPlaylist|Num (Variables|Default|GetPlayList)))
      (bind _output_get (LocalVariables|Setl_PlayListSize _returnvalue))
      (if (> _output_get 0)
        (for _index (range 0 (- (LocalVariables|Getl_PlayListSize) 1))
          (Class|MediaPlaylist|Removeat (Variables|Default|GetPlayList) _index))))
    (:then_1
      (for _array_element NewList
        (Class|MediaPlaylist|AddFile (Variables|Default|GetPlayList) _array_element)))))