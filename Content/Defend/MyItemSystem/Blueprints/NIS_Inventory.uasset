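; Slot-based inventory for the item system, storing items in an array pre-filled to InventorySize on BeginPlay.
; Each slot carries a Valid flag alongside item GUID, definition and current state.
; Functions named as server operations add to the first free slot when given a negative index, overwrite a slot, or change its amount.
; An amount of zero or less resets the slot through the set-item function.
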(event EventBeginPlay
  (for _index (range 0 (- (Variables|Default|GetInventorySize) 1))
    (Utilities|Array|Add :TargetArray (Variables|Default|GetItems))))

(fn FuncServerAddItem
  (params (NewItem :type NIS%20S%20Item%20Structure%20%28by%20ref%29) (Slot :type Integer))
  (if (< Slot 0)
    (for (_array_element _array_index) (Variables|Default|GetItems)
      (if (not (.Valid (Utilities|Struct|BreakNIS_S_Item _array_element)))
        (Utilities|Array|SetArrayElem (Variables|Default|GetItems) _array_index (Utilities|Struct|MakeNIS_S_Item true (.itemguid NewItem) (.definiation NewItem) (.currentstate NewItem)))
        (return true)))
    (return false)))

(fn FuncServerSetItem
  (params (Slot :type Integer) (ItemInfo :type NIS%20S%20Item%20Structure))
  (if (Utilities|Array|IsValidIndex (Variables|Default|GetItems) Slot)
    (Utilities|Array|SetArrayElem (Variables|Default|GetItems) Slot ItemInfo)
    (return true)
    (else
      (return false))))

(fn FuncServerSetItemAmount
  (params (Slot :type Integer) (NewAmount :type Integer))
  (bind _items (Variables|Default|GetItems))
  (bind _output (Utilities|Array|Get(acopy) _items Slot))
  (bind _currentstate (Utilities|Struct|BreakNIS_S_Item _output))
  (if (Utilities|Array|IsValidIndex (Variables|Default|GetItems) Slot)
    (if (> NewAmount 0)
      (if (.Valid (Utilities|Struct|BreakNIS_S_Item _output))
        (bind _structout (Utilities|Struct|SetmembersinNIS_S_Item _output (Utilities|Struct|MakeNIS_S_ItemCurrentState (.quality _currentstate) NewAmount (.randomizedpropbounce _currentstate))))
        (Development|PrintString (Utilities|String|ToString(Boolean) (.Valid (Utilities|Struct|BreakNIS_S_Item _structout))))
        (return true))
      (else
        (CallFunction|FuncServerSetItem Slot)))
    (else
      (return false))))