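; Equipped firearm item with ammo ID, muzzle effects and interaction-based pickup, apparently left partly gutted.
; Trigger input drives a one-shot check, fire, damage and cooldown loop that repeats while held.
; Firing cannot succeed: the can-shoot check is empty and the ammo test compares zero to zero.
; Aim, reload, pickup and the screen-centre trace with team-filtered damage, bomb spawn and voxel carving remain only as disconnected logic.
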(event Custom|CE_OneShot
  (if (CallFunction|PureCanShot)
    (bind _succ (CallFunction|FuncFiretheBullet))
    (if _succ
      (CallFunction|FuncApplyDamageonTarget)
      (Utilities|FlowControl|Delay (Variables|Default|GetCD))
      (CallFunction|FunconCooldown)
      (else
        (Audio|SpawnSoundAttached "/Game/Defend/Sounds/NoAmmo.NoAmmo" (Variables|Default|GetMuzzle) "None" "0, 0, 0" "0, 0, 0" "KeepRelativeOffset" false 1.0 1.0 0.0 0 0)
        (Rendering|SetVisibility (Variables|Default|GetParticleSystem) false false :!label _label)))
    (else
      (goto _label))))

(event Custom|I_MainAction_1
  (params (Pressed :type Boolean))
  (bind _output_get (Variables|Default|SetTriggerPressed Pressed))
  (if _output_get
    (CallFunction|CEOneShot)))

(event Custom|I_ThirdAction_1
  (params (Pressed :type Boolean)))

(event Custom|I_RecallAction_1
  (params (ActionName :type Name) (ActionBegin :type Boolean)))

(event Custom|I_SecondAction_1
  (params (Pressed :type Boolean)))

(event EventBeginPlay
  (|CallParentFunction)
  (bind _returnvalue (Utilities|GetDataTableRow "/Game/Defend/Datatables/ItemList.ItemList" (Variables|Default|GetAmmoID))))

(fn ConstructionScript
  (|CallParentFunction))

(fn PureCanShot)

(fn FuncApplyDamageonTarget)

(fn FuncFiretheBullet
  (if (> 0 0)
    (Components|Activation|SetActive (Variables|Default|GetParticleSystem) true false)
    (Rendering|SetVisibility (Variables|Default|GetParticleSystem) true false)
    (else
      (return false))))

(fn FunconCooldown
  (Variables|Default|SetCooldown true)
  (Rendering|SetVisibility (Variables|Default|GetParticleSystem) false false)
  (if (Variables|Default|GetTriggerPressed)
    (CallFunction|CEOneShot)))

(fn FuncBeenInteracted
  (params (ByWhom :type Actor%20Object%20Reference))
  (CallFunction|FuncPickup ByWhom))

(fn FuncPickup
  (params (ByWhom :type Actor%20Object%20Reference)))

(fn PureGetReloadInfo
  (Utilities|FlowControl|Sequence
    (:then_0
      (bind _output_get (LocalVariables|Setl_AmmoNeeded (- 0 1)))
      (if (> _output_get 0)
        (LocalVariables|Setl_AmmoIHave (CallFunction|PureGetAmmoinInventory (Variables|Default|GetAmmoID)))))
    (:then_1
      (return (LocalVariables|Getl_AmmoIHave) (LocalVariables|Getl_AmmoNeeded)))))

(fn PureGetAmmoinInventory
  (params (ID :type Name)))

(fn FunconRecall
  (params (ActionName :type Name) (ActionBegin :type Boolean)))

(fn IGetAmmoID
  (return (Variables|Default|GetAmmoID)))

(fn IGetAttachType
  (return "NewEnumerator0"))