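; BP_VoxelMining converts voxel terrain edits into inventory resources for the mining pawn.
; On each mined event, FuncMined sums voxel value changes by each position's strongest landscape material name.
; It parses "Resource_" IDs from those names to look up ItemList rows, setting amounts to the floored totals.
; Items go into the Pawn_L1_Equipment inventory, and failed adds spawn World_Actor items at the miner's location.
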(event Custom|CE_VoxelMined
  (params (ModifedValues :type Array%20of%20Modified%20Voxel%20Value%20Structures) (EditedBounds :type Voxel%20Int%20Box%20Structure) (Who :type Actor%20Object%20Reference%20%28by%20ref%29) (VWorld :type Voxel%20World%20Object%20Reference))
  (CallFunction|FuncMined ModifedValues EditedBounds Who VWorld))

(event EventBeginPlay)

(event Collision|EventActorBeginOverlap
  (params (OtherActor :type Actor%20Object%20Reference)))

(event EventTick
  (params (DeltaSeconds :type Float%20%28single-precision%29)))

(fn ConstructionScript)

(fn FuncMined
  (params (ModifiedValues :type Array%20of%20Modified%20Voxel%20Value%20Structures) (EditedBounds :type Voxel%20Int%20Box%20Structure) (Who :type Actor%20Object%20Reference%20%28by%20ref%29) (VWorld :type Voxel%20World%20Object%20Reference))
  (bind _l_resourcecollected (LocalVariables|Getl_ResourceCollected))
  (bind _l_resourcecollected_2 (LocalVariables|Getl_ResourceCollected))
  (for _array_element ModifiedValues
    (bind _material (Class|VoxelDataTools|GetMaterial VWorld (.Position (Utilities|Struct|BreakModifiedVoxelValue _array_element))))
    (Utilities|Map|Add _l_resourcecollected (Utilities|GetObjectName (Class|VoxelMaterialCollectionBase|GetIndexMaterial (LocalVariables|Getl_LandscapeMatCollection) (.Index0 (Class|VoxelBlueprintLibrary|GetMultiIndex _material true)))) (+ (.Value (Utilities|Map|Find _l_resourcecollected (Utilities|GetObjectName (Class|VoxelMaterialCollectionBase|GetIndexMaterial (LocalVariables|Getl_LandscapeMatCollection) (.Index0 (Class|VoxelBlueprintLibrary|GetMultiIndex _material true)))))) (- (.NewValue (Utilities|Struct|BreakModifiedVoxelValue _array_element)) (.OldValue (Utilities|Struct|BreakModifiedVoxelValue _array_element))))))
  (bind _keys (Utilities|Map|Keys _l_resourcecollected_2))
  (LocalVariables|Setl_Keys _keys)
  (bind _values (Utilities|Map|Values _l_resourcecollected_2))
  (LocalVariables|Setl_Values _values)
  (for _array_element_2 (LocalVariables|Getl_Keys)
    (bind _aspawn_l1_equipment (Utilities|Casting|CastToPawn_L1_Equipment Who))
    (for (_array_element_3 _array_index) (LocalVariables|Getl_Keys)
      (bind _returnvalue (Utilities|GetDataTableRow "/Game/Defend/Datatables/ItemList.ItemList" (CallFunction|PureMaterialNametoItemID _array_element_3))
        (:then
          (bind _output_get (LocalVariables|Setl_TempItem _returnvalue))
          (bind _structout (Utilities|Struct|SetmembersinInventoryItem _output_get (Math|Float|Floor (Utilities|Array|Get(acopy) (LocalVariables|Getl_Values) _array_index))))
          (bind (_success _outitem) (Default|TrytoAddItemtoInventory (Variables|/Game/Defend/Blueprints/Pawns/Pawn_L1_Equipment.Pawn_L1_Equipment_C|GetInventoryManagerComponent _aspawn_l1_equipment) (Variables|/Game/Defend/Blueprints/Pawns/Pawn_L1_Equipment.Pawn_L1_Equipment_C|GetEquipmentInventoryComponent _aspawn_l1_equipment) _structout))
          (if (not _success)
            (Game|SpawnActorfromClass "/Game/Defend/Blueprints/Usables/World_Actor.World_Actor_C" (Math|Transform|MakeTransform (Transformation|GetActorLocation Who) "0, 0, 0" "1,1,1") "AlwaysSpawn" 0 (.ID (Utilities|Struct|BreakInventoryItem _outitem)) (.Amount (Utilities|Struct|BreakInventoryItem _outitem)) 0)))))))

(fn PureMaterialNametoItemID
  (params (MatName :type String))
  (LocalVariables|Setl_SourceTypePos (Utilities|String|FindSubstring MatName "Resource_"))
  (if (>= (LocalVariables|Getl_SourceTypePos) 0)
    (LocalVariables|Setl_EndPos (Utilities|String|FindSubstring MatName "_" false false (+ (LocalVariables|Getl_SourceTypePos) 9)))
    (return (Utilities|String|StringToName (Utilities|String|GetSubstring MatName (LocalVariables|Getl_SourceTypePos) (- (LocalVariables|Getl_EndPos) (LocalVariables|Getl_SourceTypePos)))))
    (else
      (return "None"))))