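; Game mode for Defend that places restarted players at their own tagged start points, with support for two local players.
; On player restart, it destroys any valid controlled pawn, then spawns and possesses a Pawn_L4_PlayerPawn in its place.
; The controller ID picks the PlayerStart tag: P1 for ID 0, P2 for any other.
; A CreatePlayer call is present but unconnected, so it never runs.
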(event EventBeginPlay)

(event EventTick
  (params (DeltaSeconds :type Float%20%28single-precision%29)))

(event EventOnRestartPlayer
  (params (NewPlayer :type Controller%20Object%20Reference))
  (bind _returnvalue (Pawn|GetControlledPawn NewPlayer))
  (Utilities|IsValid _returnvalue
    (:Is%20Valid
      (Actor|DestroyActor _returnvalue)
      (bind _outactors (Actor|GetAllActorsOfClasswithTag "/Script/Engine.PlayerStart" (select (== (Class|GameplayStatics|GetPlayerControllerID (.AsPlayer%20Controller (Utilities|Casting|CastToPlayerController NewPlayer))) 0) "P1" "P2")))
      (bind _returnvalue_2 (Game|SpawnActorfromClass "/Game/Defend/Blueprints/Pawns/Pawn_L4_PlayerPawn.Pawn_L4_PlayerPawn_C" (Transformation|GetActorTransform (Utilities|Array|Get(acopy) _outactors)) "AdjustIfPossibleButAlwaysSpawn" 0 0))
      (Pawn|Possess NewPlayer _returnvalue_2))))

(fn ConstructionScript)