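; AI component for an enemy pawn (Pawn_L4_Enemy) that selects targets and steers pursuit through a state machine.
; A delayed Tick updates state, choosing among reported targets by nav path and falling back to reachable points when paths are empty or partial.
; Losing a target can queue overlapping destructibles as block targets.
; Wandering movement and the pursue-and-attack call sit in disconnected graph, alongside debug prints and spheres.
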(event Custom|CE_AI
  (Utilities|IsValid (Game|Player|GetPlayerPawn 0) :!label _label
    (:Is%20Not%20Valid
      (Utilities|FlowControl|Delay 0.2)
      (goto _label))))

(event Custom|CE_UpdateTarget
  (params (Target :type Actor%20Object%20Reference) (SenseOrForget :type Boolean) (Age :type Float%20%28single-precision%29) (MaxAge :type Float%20%28single-precision%29))
  (CallFunction|FuncUpdateTarget Target SenseOrForget Age MaxAge))

(event Custom|CE_StartPursue
  (switch Utilities|FlowControl|Switch|SwitchonE_AIState (Variables|Default|GetState)
    (:NewEnumerator1
      (if (Variables|Default|GetTargetUnreachable)
        (AI|AIMoveTo (Variables|Default|GetOwnerPawn) (Variables|Default|GetCurrentTargetLocation) 0 5.0 false :!label _label
          (:then
            (Variables|Default|SetIsAIMoving true))
          (:OnSuccess
            (Variables|Default|SetIsAIMoving false))
          (:OnFail
            (Variables|Default|SetIsAIMoving false)))
        (else
          (AI|AIMoveTo (Variables|Default|GetOwnerPawn) "0, 0, 0" (Variables|Default|GetCurrentTarget) 1e+01 false
            (:then
              (Variables|Default|SetIsAIMoving true))
            (:OnSuccess
              (Variables|Default|SetIsAIMoving false))
            (:OnFail
              (Variables|Default|SetIsAIMoving false))))))
    (:NewEnumerator4
      (goto _label))))

(event Custom|CE_LoseTargetTryToFindIt
  (CallFunction|FuncTrytoFindLosingTarget))

(event EventBeginPlay
  (bind _aspawn (Utilities|Casting|CastToPawn (Components|GetOwner))
    (:then
      (bind _output_get (Variables|Default|SetOwnerPawn _aspawn))
      (bind _aspawn_l4_enemy (Utilities|Casting|CastToPawn_L4_Enemy _output_get))
      (Variables|Default|SetAIPerception (Variables|/Game/Defend/Blueprints/Pawns/Pawn_L4_Enemy.Pawn_L4_Enemy_C|GetAIPerception _aspawn_l4_enemy))
      (bind _asaicontroller (Utilities|Casting|CastToAIController (Pawn|GetController _aspawn_l4_enemy)))
      (Variables|Default|SetAIController _asaicontroller)
      (bind _outactors (Actor|GetAllActorsOfClass "/Script/NavigationSystem.RecastNavMesh"))
      (Variables|Default|SetNavMeshActor (Utilities|Array|Get(acopy) _outactors)))
    (:CastFailed
      (Development|PrintString "AI Must Belong to Pawns"))))

(event EventTick
  (params (DeltaSeconds :type Float%20%28single-precision%29))
  (Utilities|FlowControl|Delay (Variables|Default|GetInterval))
  (CallFunction|FuncUpdateState))

(fn FuncSetState
  (params (NewState :type E_AIState%20Enum :default "NewEnumerator0"))
  (bind _output_get (LocalVariables|Setl_PreState (Variables|Default|GetState)))
  (if (Utilities|Enum|NotEqual(Enum) _output_get NewState)
    (bind _output_get_2 (Variables|Default|SetState NewState))
    (switch Utilities|FlowControl|Switch|SwitchonE_AIState _output_get_2
      (:NewEnumerator1
        (CallFunction|CEStartPursue :!label _label))
      (:NewEnumerator4
        (goto _label))
      (:NewEnumerator3
        (Variables|Default|SetStartIdleTime (Math|DateTime|Now))))))

(fn FuncUpdateTarget
  (params (Target :type Actor%20Object%20Reference%20%28by%20ref%29) (SenseOrForget :type Boolean) (Age :type Float%20%28single-precision%29) (MaxAge :type Float%20%28single-precision%29))
  (Utilities|IsValid Target
    (:Is%20Valid
      (if SenseOrForget
        (Utilities|Array|AddUnique (Variables|Default|GetTargets) Target)
        (if (Variables|Default|GetTargetUnreachable)
          _)
        (elif (> MaxAge Age) ; 是视野丢了还是听不到超过指定时间了
          (if (== (Variables|Default|GetCurrentTarget) Target) ; 如果是当前追踪的目标丢了视野
            (CallFunction|FuncUpdateState) ; 更新自身状态,追踪最后位置,或者干其他的去
            (else
              (Utilities|Array|RemoveItem (Variables|Default|GetTargets) Target :!label _label) ; 移除这个目标
            ))
          (else
            (goto _label)))))))

(fn PureGetNearestTarget
  (for _array_element (Variables|Default|GetTargets)
    (bind _output_get (LocalVariables|Setl_Distance (Math|Vector|Distance(Vector) (Transformation|GetActorLocation _array_element) (Transformation|GetActorLocation (Variables|Default|GetOwnerPawn)))))
    (if (< _output_get (LocalVariables|Getl_NearestDistance))
      (LocalVariables|Setl_NearestDistance (LocalVariables|Getl_Distance))
      (LocalVariables|Setl_Target _array_element)))
  (Utilities|IsValid (Variables|Default|GetCurrentTarget)
    (:Is%20Valid
      (Utilities|Array|Clear (Variables|Default|GetBlockTargets))
      (return (LocalVariables|Getl_Target)))
    (:Is%20Not%20Valid
      (for _array_element_2 (Variables|Default|GetBlockTargets)
        (Utilities|IsValid _array_element_2
          (:Is%20Valid
            (bind _output_get_2 (LocalVariables|Setl_Distance (Math|Vector|Distance(Vector) (Transformation|GetActorLocation _array_element_2) (Transformation|GetActorLocation (Variables|Default|GetOwnerPawn)))))
            (if (< _output_get_2 (LocalVariables|Getl_NearestDistance))
              (LocalVariables|Setl_NearestDistance (LocalVariables|Getl_Distance))
              (LocalVariables|Setl_Target _array_element_2)))))
      (return (LocalVariables|Getl_Target)))))

(fn FuncPursue
  (bind _ownerpawn (Variables|Default|GetOwnerPawn))
  (bind _currenttarget (Variables|Default|GetCurrentTarget))
  (bind _returnvalue (Transformation|GetActorLocation _ownerpawn))
  (bind _returnvalue_2 (Transformation|GetActorLocation _currenttarget))
  (bind _aspawn_l4_enemy (Utilities|Casting|CastToPawn_L4_Enemy (Variables|Default|GetOwnerPawn)))
  (LocalVariables|Setl_Enemy _aspawn_l4_enemy)
  (bind _aspawn_l4_player_pawn (Utilities|Casting|CastToPawn_L4_PlayerPawn (Variables|Default|GetCurrentTarget))
    (:then
      (LocalVariables|Setl_TargetPlayer _aspawn_l4_player_pawn)
      (if (.ReturnValue (Default|PureIsAlive (LocalVariables|Getl_TargetPlayer)))
        (if (< (Math|Vector|Distance(Vector) (Transformation|GetActorLocation (Variables|Default|GetCurrentTarget)) (Transformation|GetActorLocation (Variables|Default|GetOwnerPawn))) 1.8e+02) :!label _label
          (Default|CEAttack (LocalVariables|Getl_Enemy) (Variables|Default|GetCurrentTarget) "0, 0, 0" :!label _label_2)
          (elif (not (Variables|Default|GetIsAIMoving))
            (if (< (Math|Vector|Distance(Vector) (Math|Vector|MakeVector (.x _returnvalue_2) (.y _returnvalue_2) 0.0) (Math|Vector|MakeVector (.x _returnvalue) (.y _returnvalue) 0.0)) 1.8e+02)
              (goto _label_2)
              (else
                (CallFunction|CEStartPursue)))))
        (else
          (CallFunction|FuncUpdateTarget (Variables|Default|GetCurrentTarget) false 0.0 0.0)
          (CallFunction|FuncSetState "NewEnumerator3"))))
    (:CastFailed
      (bind _asbp_destructible (Utilities|Casting|CastToBP_Destructible (Variables|Default|GetCurrentTarget))
        (:then
          (bind _output_get (LocalVariables|Setl_TargetBlock _asbp_destructible))
          (Utilities|IsValid _output_get
            (:Is%20Valid
              (goto _label))))
        (:CastFailed
          (CallFunction|FuncSetState "NewEnumerator3"))))))

(fn FuncTrytoFindLosingTarget
  (bind _aspawn_l4_enemy (Utilities|Casting|CastToPawn_L4_Enemy (Variables|Default|GetOwnerPawn)))
  (LocalVariables|Setl_Enemy _aspawn_l4_enemy)
  (bind _output_get (LocalVariables|Setl_TargetCount (Math|Random|RandomIntegerinRange 1 3)))
  (if (> _output_get 0)
    (for _index (range 0 (- (LocalVariables|Getl_TargetCount) 1))
      (Utilities|Array|Add (LocalVariables|Getl_NearestDistance) 9999999827968.0))
    (for (_array_element _array_index) (Collision|GetOverlappingActors (Variables|/Game/Defend/Blueprints/Pawns/Pawn_L4_Enemy.Pawn_L4_Enemy_C|GetCapsule (LocalVariables|Getl_Enemy)) "/Game/Defend/Blueprints/Destructible/BP_Destructible.BP_Destructible_C" :!class /Script/Engine.PrimitiveComponent)
      (if (< _array_index (LocalVariables|Getl_TargetCount))
        (bind (_array_element_2 _array_index_2) (Utilities|Array|ForEachLoopwithBreak (LocalVariables|Getl_NearestDistance) :!label _label)
          (:LoopBody
            (if (> _array_element_2 (Math|Vector|Distance(Vector) (Transformation|GetActorLocation _array_element) (Transformation|GetActorLocation (Variables|Default|GetOwnerPawn))))
              (Utilities|Array|AddUnique (Variables|Default|GetBlockTargets) _array_element)
              (Utilities|Array|SetArrayElem (LocalVariables|Getl_NearestDistance) _array_index_2 (Math|Vector|Distance(Vector) (Transformation|GetActorLocation _array_element) (Transformation|GetActorLocation (Variables|Default|GetOwnerPawn))))
              (goto _label Break))))))
    (CallFunction|FuncSetState "NewEnumerator1")
    (else
      (CallFunction|FuncSetState "NewEnumerator3"))))

(fn FuncUpdateState
  (bind (_succ _pos) (CallFunction|PureGetLastReachablePos))
  (bind _l_findpathtotarget (LocalVariables|Getl_FindPathToTarget))
  (bind _aicontroller (Variables|Default|GetAIController))
  (bind _returnvalue (Class|AIBlueprintHelperLibrary|GetCurrentPathPoints _aicontroller))
  (switch Utilities|FlowControl|Switch|SwitchonE_AIState (Variables|Default|GetState)
    (:NewEnumerator0
      (if (or (> (Utilities|Array|Length (Variables|Default|GetTargets)) 0) (> (Utilities|Array|Length (Variables|Default|GetBlockTargets)) 0)) :!label _label
        (CallFunction|FuncTrytoFindATargetandSetState)))
    (:NewEnumerator1
      (if (Variables|Default|GetTargetUnreachable)
        (Utilities|IsValid _l_findpathtotarget
          (:Is%20Valid
            (if (not (Class|NavigationPath|IsPartial _l_findpathtotarget))
              (Variables|Default|SetTargetUnreachable false :!label _label_2)
              (CallFunction|CEStartPursue)))
          (:Is%20Not%20Valid
            (goto _label_2)))
        (elif (== (Utilities|Array|Length (Class|AIBlueprintHelperLibrary|GetCurrentPathPoints (Variables|Default|GetAIController))) 0)
          (Variables|Default|SetTargetUnreachable true)
          (if _succ
            (bind _output_get (Variables|Default|SetCurrentTargetLocation _pos))
            (Rendering|Debug|DrawDebugSphere _output_get 1e+02 12 "(R=0.842601,G=1.000000,B=0.000000,A=1.000000)" 6.0 1.0)
            (CallFunction|CEStartPursue))
          (elif (Class|AIController|HasPartialPath (Variables|Default|GetAIController))
            (Variables|Default|SetTargetUnreachable true)
            (bind _output_get_2 (Variables|Default|SetCurrentTargetLocation (Utilities|Array|Get(acopy) _returnvalue (- (Utilities|Array|Length _returnvalue) 1))))
            (Rendering|Debug|DrawDebugSphere _output_get_2 1e+02 12 "(R=1.000000,G=0.000000,B=0.000000,A=1.000000)" 6.0 1.0)
            (CallFunction|CEStartPursue)
            (else
              (Development|PrintString "Hello"))))))
    (:NewEnumerator3
      (goto _label))))

(fn PureFindTarget
  (if (> (Utilities|Array|Length (Variables|Default|GetTargets)) 0)
    (for _array_element (Variables|Default|GetTargets)
      (LocalVariables|Setl_CurTarget _array_element)
      (bind _returnvalue (Class|NavigationSystemV1|FindPathtoActorSynchronously (Transformation|GetActorLocation (Variables|Default|GetOwnerPawn)) (LocalVariables|Getl_CurTarget) 5e+01 0 0))
      (LocalVariables|Setl_NavPointCount (Utilities|Array|Length (Variables|/Script/NavigationSystem.NavigationPath|GetPathPoints _returnvalue)))
      (LocalVariables|Setl_LastNavPoint (Utilities|Array|Get(acopy) (Variables|/Script/NavigationSystem.NavigationPath|GetPathPoints _returnvalue) (- (Utilities|Array|Length (Variables|/Script/NavigationSystem.NavigationPath|GetPathPoints _returnvalue)) 1)))
      (if (or (== (LocalVariables|Getl_NavPointCount) 0) (> (Math|Vector|Distance(Vector) (LocalVariables|Getl_LastNavPoint) (Transformation|GetActorLocation (LocalVariables|Getl_CurTarget))) 1.8e+02))
        ;[1 1 1] 如果导航不到该actor,则判断最接近该actor的导航点是否为最近的一个
        (if (< (Math|Vector|Distance(Vector) (LocalVariables|Getl_LastNavPoint) (Transformation|GetActorLocation (Variables|Default|GetOwnerPawn))) (LocalVariables|Getl_TargetPosDistance))
          (LocalVariables|Setl_TargetPos (LocalVariables|Getl_LastNavPoint))
          (LocalVariables|Setl_TargetPosDistance (Math|Vector|Distance(Vector) (LocalVariables|Getl_LastNavPoint) (Transformation|GetActorLocation (Variables|Default|GetOwnerPawn)))))
        (else
          ;[1 1 1] 如果能导航得到,则看看这个目标比之前的找到的更近一些吗
          (if (< (Math|Vector|Distance(Vector) (LocalVariables|Getl_LastNavPoint) (Transformation|GetActorLocation (Variables|Default|GetOwnerPawn))) (LocalVariables|Getl_TargetDistance))
            (LocalVariables|Setl_Target (LocalVariables|Getl_CurTarget))
            (LocalVariables|Setl_TargetDistance (Math|Vector|Distance(Vector) (LocalVariables|Getl_LastNavPoint) (Transformation|GetActorLocation (Variables|Default|GetOwnerPawn))))))))
    (return true (LocalVariables|Getl_Target) (LocalVariables|Getl_TargetPos)) ; 最后如果有target有效则说明找到了一个可以导航到的actor,如果无效则用location
    (else
      (return false 0 "0, 0, 0") ; 没有任何目标,返回失败
    )))

(fn FuncTrytoFindATargetandSetState
  (bind (_succ _target _location) (CallFunction|PureFindTarget))
  (LocalVariables|Setl_TargetFound _succ)
  (LocalVariables|Setl_NewTarget _target)
  (LocalVariables|Setl_NewTargetPos _location)
  (if (LocalVariables|Getl_TargetFound)
    (Utilities|IsValid (LocalVariables|Getl_NewTarget)
      (:Is%20Valid
        (Development|PrintString (Utilities|GetDisplayName (LocalVariables|Getl_NewTarget)))
        (Variables|Default|SetCurrentTarget (LocalVariables|Getl_NewTarget))
        (CallFunction|FuncSetState "NewEnumerator1")
        (bind _returnvalue (Class|NavigationSystemV1|FindPathtoActorSynchronously (Transformation|GetActorLocation (Variables|Default|GetOwnerPawn)) (Variables|Default|GetCurrentTarget) 3e+01 (Variables|Default|GetNavMeshActor) 0))
        (Variables|Default|SetFindPathToTarget _returnvalue))
      (:Is%20Not%20Valid
        (Development|PrintString (Utilities|String|ToString(Vector) (LocalVariables|Getl_NewTargetPos)))
        (Rendering|Debug|DrawDebugSphere (LocalVariables|Getl_NewTargetPos) 3e+01 12 "(R=1.000000,G=0.000000,B=0.000000,A=1.000000)" 1.0 1.0)
        (Variables|Default|SetCurrentTargetLocation (LocalVariables|Getl_NewTargetPos))
        (CallFunction|FuncSetState "NewEnumerator4")))
    (else
      (switch Utilities|FlowControl|Switch|SwitchonE_AIState (Variables|Default|GetState)
        (:NewEnumerator1
          (CallFunction|FuncSetState "NewEnumerator4"))))))

(fn PureGetLastReachablePos
  (bind _currenttarget (Variables|Default|GetCurrentTarget))
  (bind _returnvalue (Transformation|GetActorLocation _currenttarget))
  (Utilities|IsValid (Variables|Default|GetCurrentTarget)
    (:Is%20Valid
      (bind (_outhit _returnvalue_2) (Collision|LineTraceByChannel _returnvalue (+ _returnvalue "0, 0,-20000.000000") "TraceTypeQuery1" true (Utilities|Array|MakeArray (Variables|Default|GetCurrentTarget)) "None"))
      (if _returnvalue_2
        (bind _returnvalue_3 (Class|NavigationSystemV1|FindPathtoLocationSynchronously (Transformation|GetActorLocation (Variables|Default|GetOwnerPawn)) (.Location (Collision|BreakHitResult _outhit)) 0 0))
        (LocalVariables|Setl_NavPointCount (Utilities|Array|Length (Variables|/Script/NavigationSystem.NavigationPath|GetPathPoints _returnvalue_3)))
        (LocalVariables|Setl_LastNavPoint (Utilities|Array|Get(acopy) (Variables|/Script/NavigationSystem.NavigationPath|GetPathPoints _returnvalue_3) (- (Utilities|Array|Length (Variables|/Script/NavigationSystem.NavigationPath|GetPathPoints _returnvalue_3)) 1)))
        (if (== (LocalVariables|Getl_NavPointCount) 0)
          (return false "0, 0, 0")
          (else
            (return true (LocalVariables|Getl_LastNavPoint))))
        (else
          _)))
    (:Is%20Not%20Valid
      _))
  (return false "0, 0, 0"))