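; AI input component that drives an enemy pawn through wandering, pursuing an actor, pursuing a location and idling states.
; Sensing events maintain the target list, choosing the nearest when acquiring and switching to the last seen location when the current one is lost.
; Each tick updates state, feeds a direction into character movement, and attacks when near the target or stuck for a while, detected by low velocity.
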(event Custom|CE_UpdateTarget
  (params (SenseInfo :type Actor%20Perception%20Update%20Info%20Structure))
  (CallFunction|FuncUpdateTarget SenseInfo))

(event EventTick
  (params (DeltaSeconds :type Float%20%28single-precision%29))
  (CallFunction|FuncUpdateState)
  (CallFunction|FuncInput))

(fn FuncSetState
  (params (NewState :type E_AIState%20Enum :default "NewEnumerator0"))
  (bind _output_get (LocalVariables|Setl_PreState (Variables|Default|GetState)))
  (if (Utilities|Enum|NotEqual(Enum) _output_get NewState)
    (bind _output_get_2 (Variables|Default|SetState NewState))
    (Utilities|Array|SetArrayElem (Variables|Default|GetStateStartTimes) (Math|Conversions|ToInteger(Byte) _output_get_2) (Math|DateTime|Now) true)))

(fn FuncUpdateTarget
  (params (SenseInfo :type Actor%20Perception%20Update%20Info%20Structure))
  (if (> (.expirationage (.stimulus SenseInfo)) 9e+01) ; 是视野目标变化吗?
    (if (.bsuccessfullysensed (.stimulus SenseInfo)) ; 目标进入视野?
      (Utilities|Array|AddUnique (Variables|Default|GetTargets) (.target SenseInfo))
      (switch Utilities|FlowControl|Switch|SwitchonE_AIState (Variables|Default|GetState)
        (:NewEnumerator0
          _)
        (:NewEnumerator4
          _)
        (:NewEnumerator3
          _))
      (Variables|Default|SetCurrentTarget (CallFunction|PureGetNearestTarget))
      (CallFunction|FuncSetState "NewEnumerator1")
      (else
        (Utilities|Array|RemoveItem (Variables|Default|GetTargets) (.target SenseInfo)) ; 移除这个目标
        (switch Utilities|FlowControl|Switch|SwitchonE_AIState (Variables|Default|GetState)
          (:NewEnumerator1
            (if (== (Variables|Default|GetCurrentTarget) (.target SenseInfo)) ; 如果是当前追踪的目标丢了视野
              (Variables|Default|SetCurrentTargetLocation (.stimuluslocation (.stimulus SenseInfo)))
              (Variables|Default|SetCurrentTarget 0)
              (CallFunction|FuncSetState "NewEnumerator4"))))))))

(fn PureGetNearestTarget
  (for _array_element (Variables|Default|GetTargets)
    (bind _output_get (LocalVariables|Setl_Distance (Math|Vector|Distance(Vector) (Transformation|GetActorLocation _array_element) (Transformation|GetActorLocation (Variables|Default|GetOwnerPawn)))))
    (if (< _output_get (LocalVariables|Getl_NearestDistance))
      (LocalVariables|Setl_NearestDistance (LocalVariables|Getl_Distance))
      (LocalVariables|Setl_Target _array_element)))
  (Utilities|IsValid (Variables|Default|GetCurrentTarget)
    (:Is%20Valid
      (Utilities|Array|Clear (Variables|Default|GetBlockTargets))
      (return (LocalVariables|Getl_Target)))
    (:Is%20Not%20Valid
      (for _array_element_2 (Variables|Default|GetBlockTargets)
        (Utilities|IsValid _array_element_2
          (:Is%20Valid
            (bind _output_get_2 (LocalVariables|Setl_Distance (Math|Vector|Distance(Vector) (Transformation|GetActorLocation _array_element_2) (Transformation|GetActorLocation (Variables|Default|GetOwnerPawn)))))
            (if (< _output_get_2 (LocalVariables|Getl_NearestDistance))
              (LocalVariables|Setl_NearestDistance (LocalVariables|Getl_Distance))
              (LocalVariables|Setl_Target _array_element_2)))))
      (return (LocalVariables|Getl_Target)))))

(fn FuncUpdateState
  (switch Utilities|FlowControl|Switch|SwitchonE_AIState (Variables|Default|GetState)
    (:NewEnumerator1
      (if (< (Math|Vector|VectorLength (Pawn|Components|CharacterMovement|GetLastUpdateVelocity (Variables|Default|GetOwnerCharacterMovement))) 5e+01)
        (if (not (Variables|Default|GetMayBlocked))
          (Variables|Default|SetMayBlocked true)
          (Variables|Default|SetBlockStartTime (Math|DateTime|Now))
          (Variables|Default|SetBlockLocation (Transformation|GetActorLocation (Variables|Default|GetOwnerPawn))))
        (elif (Variables|Default|GetMayBlocked)
          (if (> (Math|Vector|Distance(Vector) (Variables|Default|GetBlockLocation) (Transformation|GetActorLocation (Variables|Default|GetOwnerPawn))) 2.5e+02)
            (Variables|Default|SetMayBlocked false)))))
    (:NewEnumerator4
      (if (and (> (Math|Timespan|GetTotalSeconds (- (Math|DateTime|Now) (Utilities|Array|Get(acopy) (Variables|Default|GetStateStartTimes) (Math|Conversions|ToInteger(Byte) (Variables|Default|GetState))))) 1e+01) (> (Math|Vector|Distance(Vector) (Variables|Default|GetCurrentTargetLocation) (Transformation|GetActorLocation (Variables|Default|GetOwnerPawn))) 1.5e+03))
        (CallFunction|FuncSetState "NewEnumerator3")))))

(fn FuncInput
  (Class|PawnMovementComponent|AddInputVector (Variables|Default|GetOwnerCharacterMovement) (CallFunction|PureGetMoveDir) false)
  (switch Utilities|FlowControl|Switch|SwitchonE_AIState (Variables|Default|GetState)
    (:NewEnumerator1
      (if (or (and (>= (Math|Timespan|GetTotalSeconds (- (Math|DateTime|Now) (Variables|Default|GetBlockStartTime))) 2.0) (Variables|Default|GetMayBlocked)) (< (Math|Vector|Distance(Vector) (Transformation|GetActorLocation (Variables|Default|GetCurrentTarget)) (Transformation|GetActorLocation (Variables|Default|GetOwnerPawn))) 2.5e+02))
        (bind _aspawn_l4_enemy (Utilities|Casting|CastToPawn_L4_Enemy (Variables|Default|GetOwnerPawn)))
        (Default|CEAttack _aspawn_l4_enemy 0 "0, 0, 0")))))

(fn PureGetMoveDir
  (bind _ownerpawn (Variables|Default|GetOwnerPawn))
  (bind _returnvalue (Transformation|GetActorLocation _ownerpawn))
  (switch Utilities|FlowControl|Switch|SwitchonE_AIState (Variables|Default|GetState)
    (:NewEnumerator0
      (return (Math|Vector|MakeVector 0.0 0.0 (Math|Random|RandomFloatinRange -1.8e+02 1.8e+02))))
    (:NewEnumerator1
      (return (Math|Vector|Normalize (- (Transformation|GetActorLocation (Variables|Default|GetCurrentTarget)) _returnvalue) 0.0)))
    (:NewEnumerator4
      (return (Math|Vector|Normalize (- (Variables|Default|GetCurrentTargetLocation) _returnvalue) 0.0)))
    (:NewEnumerator3
      (return "0, 0,0.000000"))))