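; Zombie enemy pawn that chooses targets through AI perception, fed to CInputAI, and claws destructibles or opposing-team players.
; Attacks play a montage facing the target, and right-hand collision overlap deals damage, then disables itself.
; On death it expires shortly and may drop rifle ammo split into random pickups.
; When AI-controlled, it derives animation movement input from velocity; Tick and perception updates also emit debug output.
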(event OnComponentBeginOverlap(MeleeCollisionHandR)
  (params (OverlappedComponent :type Primitive%20Component%20Object%20Reference) (OtherActor :type Actor%20Object%20Reference) (OtherComp :type Primitive%20Component%20Object%20Reference) (OtherBodyIndex :type Integer) (bFromSweep :type Boolean) (SweepResult :type Hit%20Result%20Structure%20%28by%20ref%29))
  (CallFunction|FuncHitSomething OtherActor (Transformation|GetWorldLocation OverlappedComponent)))

(event OnTargetPerceptionInfoUpdated(AIPerception)
  (params (UpdateInfo :type Actor%20Perception%20Update%20Info%20Structure%20%28by%20ref%29))
  (bind (_targetid _target _stimulus) (Utilities|Struct|BreakActorPerceptionUpdateInfo UpdateInfo))
  (bind (_age _expirationage _strength _stimuluslocation _receiverlocation _tag _bsuccessfullysensed) (Utilities|Struct|BreakAIStimulus _stimulus))
  (Default|CEUpdateTarget (Variables|Default|GetC_InputAI) UpdateInfo)
  (Rendering|Debug|DrawDebugSphere _stimuluslocation 5e+01 12 (Math|Color|SelectColor "(R=0.000000,G=0.207691,B=1.000000,A=1.000000)" "(R=1.000000,G=0.000000,B=0.000000,A=1.000000)" _bsuccessfullysensed) 1.0 1.0)
  (Development|PrintString (Utilities|GetDisplayName _target)))

(event Custom|CE_Attack
  (params (Target :type Actor%20Object%20Reference) (HitPoint :type Vector))
  (CallFunction|FuncAttack Target HitPoint))

(event EventBeginPlay
  (|CallParentFunction)
  (Variables|/Game/Defend/Blueprints/Pawns/C_InputAI.C_InputAI_C|SetOwnerPawn (Variables|Default|GetC_InputAI) self)
  (Variables|/Game/Defend/Blueprints/Pawns/C_InputAI.C_InputAI_C|SetAIPerception (Variables|Default|GetC_InputAI) (Variables|Default|GetAIPerception))
  (Variables|/Game/Defend/Blueprints/Pawns/C_InputAI.C_InputAI_C|SetOwnerCharacterMovement (Variables|Default|GetC_InputAI) (Variables|Character|GetCharacterMovement)))

(event EventTick
  (params (DeltaSeconds :type Float%20%28single-precision%29))
  (bind _mesh (Variables|Character|GetMesh))
  (bind _returnvalue (Components|SkeletalMesh|GetAnimInstance _mesh))
  (|CallParentFunction DeltaSeconds)
  (for _array_element (Class|AnimInstance|GetAllCurveNames _returnvalue)
    (Development|PrintString (Utilities|String|Append (Utilities|String|ToString(Name) _array_element) ":" (Utilities|String|ToString(Text) (Utilities|Text|ToText(Float) (Animation|Curves|GetCurveValue _returnvalue _array_element) "HalfToEven" false true 1 324 1 1))) true true "(R=0.000000,G=0.660000,B=1.000000,A=1.000000)" 0.02)))

(event EventIMeleeAttack
  (params (Begin :type Boolean))
  (Variables|Default|SetIsMeleeAttacking Begin))

(fn ConstructionScript
  (Variables|/Script/Engine.CharacterMovementComponent|SetMaxWalkSpeed (Variables|Character|GetCharacterMovement) (Variables|Default|GetZombieMovementSpeed)))

(fn FuncAttack
  (params (TargetActor :type Actor%20Object%20Reference) (HitPoint :type Vector))
  (bind _movementaction (Variables|Default|GetMovementAction))
  (if (Math|Boolean|ANDBoolean (Utilities|Enum|NotEqual(Enum) _movementaction "NewEnumerator5") (Utilities|Enum|NotEqual(Enum) _movementaction "NewEnumerator3") (Utilities|Enum|Equal(Enum) (Variables|Default|GetMovementState) "NewEnumerator1") (not (Variables|Default|GetIsMeleeAttacking)) (.ReturnValue (CallFunction|PureIsAlive)))
    (bind _mainaniminstance (Variables|Default|GetMainAnimInstance)
      (:then
        (Animation|Montage|MontagePlay _mainaniminstance "/Game/Defend/Animations/Zombie/Montages/AM_Z_Attack.AM_Z_Attack" 1.0 "MontageLength" 0.1 true)
        (Utilities|IsValid TargetActor
          (:Is%20Valid
            (Transformation|SetActorRotation (Math|Rotator|MakeRotfromXZ (Math|Vector|ProjectVectorontoPlane (- (Transformation|GetActorLocation TargetActor) (Transformation|GetActorLocation)) "0, 0,1.000000") (Math|Vector|MakeVector 0.0 0.0 1.0)) true))))
      (:else))))

(fn FuncHitSomething
  (params (ActorHit :type Actor%20Object%20Reference) (ImpreciseHitLocation :type Vector))
  (bind _asbp_destructible (Utilities|Casting|CastToBP_Destructible ActorHit)
    (:then
      (Default|ITakeDamage _asbp_destructible (Variables|Default|GetZombieClawDamage) "NewEnumerator0" self ImpreciseHitLocation)
      (Collision|SetCollisionEnabled (Variables|Default|GetMeleeCollisionHandR) "NoCollision"))
    (:CastFailed
      (bind _aspawn_l4_player_pawn (Utilities|Casting|CastToPawn_L4_PlayerPawn ActorHit))
      (bind _id (Default|IGetTeamID _aspawn_l4_player_pawn))
      (if (!= _id (Variables|Default|GetTeamID))
        (Default|ITakeDamage _aspawn_l4_player_pawn (Variables|Default|GetZombieClawDamage) "NewEnumerator0" self ImpreciseHitLocation)
        (Collision|SetCollisionEnabled (Variables|Default|GetMeleeCollisionHandR) "NoCollision")))))

(fn FunconMeleeCollisionEnable
  (params (Enable :type Boolean) (CollisionSockName :type Name :default "None"))
  (|CallParentFunction Enable CollisionSockName)
  (Collision|SetCollisionEnabled (Variables|Default|GetMeleeCollisionHandR) (select Enable "QueryOnly" "NoCollision")))

(fn FuncDie
  (|CallParentFunction)
  (Actor|SetLifeSpan 3.0)
  (if (< (Math|Random|RandomFloatinRange 0.0 1e+02) 5e+01)
    (bind _output_get (LocalVariables|Setl_Amount (Math|Random|RandomIntegerinRange 10 80)))
    (while (> _output_get 0)
      (LocalVariables|Setl_Spawned (Math|Random|RandomIntegerinRange (Math|Integer|Min(Integer) (LocalVariables|Getl_Amount) 5) (Math|Integer|Min(Integer) (LocalVariables|Getl_Amount) 30)))
      (Game|SpawnActorfromClass "/Game/Defend/Blueprints/Usables/World_Actor.World_Actor_C" (Math|Transform|MakeTransform (Transformation|GetActorLocation) "0, 0, 0" "1,1,1") "Undefined" 0 "Ammo_Rifle" (LocalVariables|Getl_Spawned) 0)
      (bind _output_get_2 (LocalVariables|Setl_Amount (- (stale _output_get_2) (LocalVariables|Getl_Spawned)))))))

(fn BPIGetEssentialValues
  (if (Pawn|IsPlayerControlled)
    (bind (_velocity _acceleration _movementinput _ismoving _hasmovementinput _speed _movementinputamount _aimingrotation _aimyawrate) (|CallParentFunction))
    (return _velocity _acceleration _movementinput _ismoving _hasmovementinput _speed _movementinputamount _aimingrotation _aimyawrate)
    (else
      (bind (_velocity_2 _acceleration_2 _movementinput_2 _ismoving_2 _hasmovementinput_2 _speed_2 _movementinputamount_2 _aimingrotation_2 _aimyawrate_2) (|CallParentFunction))
      (return _velocity_2 _acceleration_2 (Math|Vector|Normalize _velocity_2 0.0) _ismoving_2 (> _speed_2 0.0) _speed_2 (Math|Float|SelectFloat 1.0 0.0 (> _speed_2 0.0)) _aimingrotation_2 _aimyawrate_2))))