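; BP_Door is a usable, destructible door that toggles open and closed when used.
; OnWasUsed triggers a FlipFlop that snaps RotRoot between open and closed rotations without animation.
; The construction script assigns destructible meshes to door and frame before running the parent's script.
; BeginPlay binds a destruction handler, but it is empty; the cleanup for meshes, trigger collision and nav modifiers is disconnected.
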(event Custom|CE_SwitchDoor
  (bind _rotroot (Variables|Default|GetRotRoot))
  (Utilities|FlowControl|FlipFlop
    (:A
      (Transformation|SetRelativeRotation _rotroot "0,120.000000, 0" false false))
    (:B
      (Transformation|SetRelativeRotation _rotroot "0, 0, 0" false false))))

(event Custom|BE_OnDestroy)

(event EventBeginPlay
  (|CallParentFunction)
  (EventDispatchers|BindEventtoEDonDestruction (delegate Custom|BE_OnDestroy)))

(event Collision|EventActorBeginOverlap
  (params (OtherActor :type Actor%20Object%20Reference)))

(event EventTick
  (params (DeltaSeconds :type Float%20%28single-precision%29)))

(fn ConstructionScript
  (Class|DestructibleComponent|SetDestructibleMesh (Variables|Default|GetDM_Door) "/Game/Defend/Blueprints/Destructible/Door/SM_Door_DM.SM_Door_DM")
  (Class|DestructibleComponent|SetDestructibleMesh (Variables|Default|GetDM_Frame) "/Game/Defend/Blueprints/Destructible/Door/SM_DoorFrame_DM.SM_DoorFrame_DM")
  (|CallParentFunction))

(fn OnWasUsed
  (CallFunction|CESwitchDoor)
  (return false))