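; BP_Block is an experimental procedural-mesh block under Destructible, with all its logic currently disconnected, including the construction script and FuncModifyCube.
; Unwired experiments build a cube from eight vertices or per-face UV sections, or copy a static mesh into the procedural mesh.
; Further unwired code offsets coincident vertices together to reshape corners and edges, then rebuilds convex collision.
; Debug spheres and vertex-index widgets visualise the geometry.
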(fn ConstructionScript)

(fn PureGetFace
  (params (Index :type Integer))
  (bind _vertices (Variables|Default|GetVertices))
  (bind _vertices_2 (Variables|Default|GetVertices))
  (switch int Index
    (:0
      (return (Utilities|Array|MakeArray (Utilities|Array|Get(acopy) _vertices_2) (Utilities|Array|Get(acopy) _vertices_2 1) (Utilities|Array|Get(acopy) _vertices_2 2) (Utilities|Array|Get(acopy) _vertices_2 3)) (Utilities|Array|MakeArray 0 1 2 2 3 0) (Utilities|Array|MakeArray "(X=0.000000,Y=1.000000)" "(X=0.000000,Y=0.000000)" "(X=1.000000,Y=0.000000)" "(X=1.000000,Y=1.000000)")))
    (:1
      (return (Utilities|Array|MakeArray (Utilities|Array|Get(acopy) _vertices 4) (Utilities|Array|Get(acopy) _vertices 5) (Utilities|Array|Get(acopy) _vertices 6) (Utilities|Array|Get(acopy) _vertices 7)) (Utilities|Array|MakeArray 0 2 1 2 0 3) (Utilities|Array|MakeArray "(X=0.000000,Y=0.000000)" "(X=1.000000,Y=0.000000)" "(X=1.000000,Y=1.000000)" "(X=0.000000,Y=1.000000)")))))

(fn FuncOffsetAVertex
  (params (Index :type Integer) (Offset :type Vector) (AllVertices :type Boolean))
  (bind _output_get (LocalVariables|Setl_TargetVertexPos (Utilities|Array|Get(acopy) (Variables|Default|GetVertices) Index)))
  (LocalVariables|Setl_NewVertexPos (+ _output_get Offset))
  (if AllVertices
    (for (_array_element _array_index) (Variables|Default|GetVertices)
      (LocalVariables|Setl_CurIDX _array_index)
      (if (Math|Vector|Equal(Vector) _array_element (LocalVariables|Getl_TargetVertexPos) 1.0)
        (|SetBy-RefVar (Utilities|Array|Get(acopy) (Variables|Default|GetVertices) (LocalVariables|Getl_CurIDX)) (LocalVariables|Getl_NewVertexPos))))
    (else
      (|SetBy-RefVar (Utilities|Array|Get(acopy) (Variables|Default|GetVertices) Index) (LocalVariables|Getl_NewVertexPos)))))

(fn FuncModifyCube
  (params (Index :type Integer) (Offset :type Vector) (AllVertices :type Boolean)))