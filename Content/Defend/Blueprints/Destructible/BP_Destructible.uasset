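; Destructible actor that takes damage through a TakeDamage interface, tracking health from a configurable maximum.
; Construction swaps destructible component materials for dynamic instances, whose DamageRate parameter rises as health falls.
; Each hit also plays a sound at its location and calls an empty mesh-update function.
; At zero health it fires an OnDestruction dispatcher once and destroys itself; the mesh-fracture and collapse-sound logic is disconnected.
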(event EventBeginPlay
  (Variables|Default|SetHealth (Variables|Default|GetMaxHealth)))

(event EventITakeDamage
  (params (Amount :type Float%20%28single-precision%29) (Type :type E_DamageType%20Enum :default "NewEnumerator0") (Instigator :type Actor%20Object%20Reference) (Location :type Vector :default "0, 0, 0"))
  (CallFunction|FuncModHealth Amount)
  (Rendering|Material|SetScalarParameterValue (Variables|Default|GetMI_Materials) "DamageRate" (- 1.0 (CallFunction|PureGetHealthPercent)) :!class /Script/Engine.MaterialInstanceDynamic)
  (Audio|PlaySoundatLocation (Variables|Default|GetHitSound) Location "0, 0, 0" 1.0 1.0 0.0 0 0 0)
  (CallFunction|FuncUpdateMeshandMat)
  (if (CallFunction|PureIsDead)
    (Utilities|FlowControl|DoOnce false
      (:Completed
        (Default|CallEDonDestruction)
        (Actor|DestroyActor)))))

(fn ConstructionScript
  (Utilities|FlowControl|Sequence
    (:then_1
      (for _array_element (Actor|GetComponentsByClass "/Script/ApexDestruction.DestructibleComponent")
        (for (_array_element_2 _array_index) (Rendering|Material|GetMaterials _array_element)
          (bind _returnvalue (Rendering|Material|CreateDynamicMaterialInstance _array_element_2 "None" "None" :!class /Script/Engine.KismetMaterialLibrary))
          (Utilities|Array|Add (Variables|Default|GetMI_Materials) _returnvalue)
          (Rendering|Material|SetScalarParameterValue _returnvalue "DamageRate" 0.0 :!class /Script/Engine.MaterialInstanceDynamic)
          (Rendering|Material|SetMaterial _array_element _array_index _returnvalue))))))

(fn PureIsDead
  (return (<= (Variables|Default|GetHealth) 0.0)))

(fn FuncUpdateMeshandMat)

(fn PureGetHealthPercent
  (return (/ (Variables|Default|GetHealth) (Variables|Default|GetMaxHealth))))

(fn FuncModHealth
  (params (HealthLost :type Float%20%28single-precision%29))
  (bind _output_get (Variables|Default|SetHealth (Math|Float|Clamp(Float) (- (stale _output_get) HealthLost) 0.0 (Variables|Default|GetHealth)))))