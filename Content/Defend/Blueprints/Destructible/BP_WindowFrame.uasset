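; BP_WindowFrame is a destructible window frame actor that breaks apart all four of its sides when destroyed.
; On BeginPlay it runs the parent logic and binds BE_Destroy to the EDOnDestruction event dispatcher.
; When the dispatcher fires, BE_Destroy calls FuncDestroyMesh on the down, right, left and up frame pieces in turn.
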(event Custom|BE_Destroy
  (CallFunction|FuncDestroyMesh (Variables|Default|GetFrameDown))
  (CallFunction|FuncDestroyMesh (Variables|Default|GetFrameRight))
  (CallFunction|FuncDestroyMesh (Variables|Default|GetFrameLeft))
  (CallFunction|FuncDestroyMesh (Variables|Default|GetFrameUp)))

(event EventBeginPlay
  (|CallParentFunction)
  (EventDispatchers|BindEventtoEDonDestruction (delegate Custom|BE_Destroy)))

(event Collision|EventActorBeginOverlap
  (params (OtherActor :type Actor%20Object%20Reference))
  (|CallParentFunction OtherActor) ; This node is disabled and will not be called.\nDrag off pins to build functionality.
)

(event EventTick
  (params (DeltaSeconds :type Float%20%28single-precision%29))
  (|CallParentFunction DeltaSeconds) ; This node is disabled and will not be called.\nDrag off pins to build functionality.
)

(fn ConstructionScript
  (|CallParentFunction))