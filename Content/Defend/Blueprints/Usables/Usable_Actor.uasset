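; Usable_Actor is a base interactable actor that pawns can focus on and use.
; Focus toggles custom depth on its skeletal and static meshes for an outline, and it reports usability plus an action-and-name prompt.
; On use, only the authority toggles WasUsed, whose OnRep calls OnWasUsed to play an optional sound at the actor's location.
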(event EventBeginPlay
  (|CallParentFunction))

(fn ConstructionScript
  (|CallParentFunction))

(fn OnRepWasUsed
  (CallFunction|OnWasUsed))

(fn OnWasUsed
  (bind _usedsound (Variables|Properties|GetUsedSound))
  (Utilities|IsValid _usedsound
    (:Is%20Valid
      (Audio|PlaySoundatLocation _usedsound (Transformation|GetActorLocation) "0, 0, 0" 1.0 1.0 0.0 0 0 0))
    (:Is%20Not%20Valid
      _))
  (return true))

(fn BeginOutlineFocus
  (Rendering|SetRenderCustomDepth (Variables|Default|GetSkeletalMesh) true)
  (return true))

(fn EndOutlineFocus
  (Rendering|SetRenderCustomDepth (Variables|Default|GetSkeletalMesh) false)
  (return true))

(fn GetIsActorUsable
  (return (Variables|Properties|GetIsUsable)))

(fn GetUseActionText
  (return (Utilities|Text|FormatText "{action} {name}" (Variables|Properties|GetAction) (Utilities|Text|ToText(Name) (Variables|Properties|GetName)))))

(fn OnActorUsed
  (params (Pawn :type Pawn%20Object%20Reference))
  (Networking|SwitchHasAuthority
    (:Authority
      (if (Variables|Properties|GetWasUsed)
        (Variables|Properties|SetWasUsed false)
        (else
          (Variables|Properties|SetWasUsed true)))
      (return true))
    (:Remote
      (return false))))