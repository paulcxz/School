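; Equippable pickaxe that mines, repairs and builds voxel terrain and deals melee damage to non-teammates within range.
; Main action has the owner play a Pickaxe action whose recall traces from screen center, repeating on cooldown while held.
; Voxel hits carve a sphere, report to BP_VoxelMining and spawn physics parts from loose chunks.
; Secondary action reverts voxels to generated terrain; third action adds a sphere.
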(event Custom|CE_OneShot
  (if (CallFunction|PureCanShot)
    (Variables|Default|SetCooldown false)
    (Class|IHandEquipmentRelative|IRecallAction(Message) (Variables|Default|GetItemOwner) "Pickaxe" true)
    (Utilities|FlowControl|Delay (Variables|Default|GetCD))
    (CallFunction|FunconCooldown)))

(event Custom|CE_ApplyPhysicsToVoxelWorld
  (params (World :type Voxel%20World%20Object%20Reference) (Bounds :type Voxel%20Int%20Box%20Structure))
  (bind _results (Class|VoxelPhysicsTools|ApplyVoxelPhysics World Bounds (Variables|Default|GetPartSpawner)))
  (for _array_element _results
    (bind _asvoxel_physics_part_spawner_result_voxel_worlds (Utilities|Casting|CastToVoxelPhysicsPartSpawnerResult_VoxelWorlds _array_element))
    (Class|VoxelWorld|SetCollisionResponsetoChannel (Variables|/Script/Voxel.VoxelPhysicsPartSpawnerResult_VoxelWorlds|GetVoxelWorld _asvoxel_physics_part_spawner_result_voxel_worlds) "ECC_Pawn" "ECR_Overlap")))

(event EventBeginPlay
  (|CallParentFunction)
  (bind _returnvalue (Game|ConstructObjectfromClass self "/Script/Voxel.VoxelPhysicsPartSpawner_VoxelWorlds"))
  (Variables|Default|SetPartSpawner _returnvalue))

(event EventIMainAction
  (params (Pressed :type Boolean))
  (bind _output_get (Variables|Default|SetTriggerPressed Pressed))
  (if _output_get
    (CallFunction|CEOneShot)))

(event EventIThirdAction
  (params (Pressed :type Boolean))
  (if Pressed
    (if (CallFunction|PureCanShot)
      (Variables|Default|SetCooldown false)
      (CallFunction|FuncAddtoTarget)
      (Utilities|FlowControl|Delay (Variables|Default|GetCD))
      (Variables|Default|SetCooldown true))))

(event EventIRecallAction
  (params (ActionName :type Name :default "None") (ActionBegin :type Boolean))
  (CallFunction|FunconRecall ActionName ActionBegin))

(event EventIEquiped
  (params (Who :type Pawn%20L1%20Equipment%20Object%20Reference))
  (Class|IHandEquipmentRelative|IRecallAction(Message) (Variables|Default|GetItemOwner) "Aim" true))

(event EventISecondAction
  (params (Pressed :type Boolean))
  (if Pressed
    (if (CallFunction|PureCanShot)
      (Variables|Default|SetCooldown false)
      (CallFunction|FuncRepairTarget)
      (Utilities|FlowControl|Delay (Variables|Default|GetCD))
      (Variables|Default|SetCooldown true))))

(event EventIUnequiped
  (params (Who :type Pawn%20L1%20Equipment%20Object%20Reference))
  (Class|IHandEquipmentRelative|IRecallAction(Message) (Variables|Default|GetItemOwner) "Aim" false))

(fn ConstructionScript
  (|CallParentFunction))

(fn PureCanShot
  (return (Variables|Default|GetCooldown)))

(fn FuncApplyDamageonTarget
  (bind _asplayer_controller (CallFunction|PureGetOwnerPC))
  (bind _itemowner (Variables|Default|GetItemOwner))
  (bind _array (Utilities|Array|MakeArray _itemowner))
  (bind (_hitresult _returnvalue) (Class|CXZFuncLib|CXZLineTracefromScreenPosPercentage _asplayer_controller "TraceTypeQuery1" _array true true 0.5 0.5))
  (bind (_bblockinghit _binitialoverlap _time _distance _location _impactpoint _normal _impactnormal _physmat _hitactor) (Collision|BreakHitResult _hitresult))
  (Utilities|IsValid _asplayer_controller
    (:Is%20Valid
      (if _returnvalue
        (bind _output_get (LocalVariables|Setl_HitLocation _location))
        (Rendering|Debug|DrawDebugSphere _output_get 1e+01 12 "(R=1.000000,G=0.000000,B=0.000000,A=1.000000)" 3.0 1.0)
        (LocalVariables|Setl_HitActor _hitactor)
        (LocalVariables|Setl_HitDistance (Math|Vector|Distance(Vector) (LocalVariables|Getl_HitLocation) (Transformation|GetWorldLocation (Variables|Default|GetStaticMesh))))
        (bind _asvoxel_world (Utilities|Casting|CastToVoxelWorld (LocalVariables|Getl_HitActor))
          (:then
            (LocalVariables|Setl_VoxelWorld _asvoxel_world)
            (if (<= (LocalVariables|Getl_HitDistance) (Variables|Default|GetMaxDistanceVoxel))
              (bind (_modifiedvalues _editedbounds) (Class|VoxelSphereTools|RemoveSphere (LocalVariables|Getl_VoxelWorld) (LocalVariables|Getl_HitLocation) (* (Variables|/Script/Voxel.VoxelWorld|GetVoxelSize (LocalVariables|Getl_VoxelWorld)) 1.5)))
              (CallFunction|FuncReportMining _modifiedvalues _editedbounds (Variables|Default|GetItemOwner) (LocalVariables|Getl_VoxelWorld))
              (CallFunction|CEApplyPhysicstoVoxelWorld (LocalVariables|Getl_VoxelWorld) (Class|VoxelBlueprintLibrary|MakeIntBoxfromGlobalPositionandRadius (LocalVariables|Getl_VoxelWorld) (LocalVariables|Getl_HitLocation) 8e+02))
              (return true)
              (else
                (return false))))
          (:CastFailed
            (if (<= (LocalVariables|Getl_HitDistance) (Variables|Default|GetMaxDistanceOther))
              (if (Utilities|DoesObjectImplementInterface (LocalVariables|Getl_HitActor) "/Game/Defend/Blueprints/Interfaces/I_Team.I_Team_C")
                (bind _id (Class|ITeam|IGetTeamID(Message) (LocalVariables|Getl_HitActor)))
                (if (!= _id (Variables|Default|GetTeamID))
                  _
                  (else
                    (return true))))
              (Class|IDamageable|ITakeDamage(Message) (LocalVariables|Getl_HitActor) (Utilities|Struct|BreakS_Properties (Default|PureGetProperties (.AsPawn%20L2%20Adv%20Locom (Utilities|Casting|CastToPawn_L2_AdvLocom (Variables|Default|GetItemOwner))))) "NewEnumerator4" (Variables|Default|GetItemOwner) "0, 0, 0")
              (return true)
              (else
                (return false)))))
        (else
          _)))
    (:Is%20Not%20Valid
      _))
  (return false))

(fn FunconCooldown
  (Variables|Default|SetCooldown true)
  (if (Variables|Default|GetTriggerPressed)
    (CallFunction|CEOneShot)))

(fn FuncBeenInteracted
  (params (ByWhom :type Actor%20Object%20Reference))
  (|CallParentFunction ByWhom)
  (CallFunction|FuncPickup ByWhom))

(fn FuncPickup
  (params (ByWhom :type Actor%20Object%20Reference))
  (bind _skeletalmesh (Variables|Default|GetSkeletalMesh))
  (bind _staticmesh (Variables|Default|GetStaticMesh))
  (|CallParentFunction ByWhom)
  (Utilities|FlowControl|Sequence
    (:then_0
      (Physics|SetSimulatePhysics _skeletalmesh false)
      (Collision|SetCollisionEnabled _skeletalmesh "NoCollision")
      (Transformation|AttachComponentToComponent (Variables|Default|GetSkeletalMesh) (Variables|Default|GetMeshRoot) "None" "SnapToTarget" "SnapToTarget" "SnapToTarget" true)
      (Transformation|SetRelativeTransform (Variables|Default|GetSkeletalMesh) (Math|Transform|MakeTransform "0, 0, 0" "0, 0, 0" "1.000000,1.000000,1.000000") false false))
    (:then_1
      (Physics|SetSimulatePhysics _staticmesh false)
      (Collision|SetCollisionEnabled _staticmesh "NoCollision")
      (Transformation|AttachComponentToComponent (Variables|Default|GetStaticMesh) (Variables|Default|GetMeshRoot) "" "SnapToTarget" "SnapToTarget" "SnapToTarget" true)
      (Transformation|SetRelativeTransform (Variables|Default|GetStaticMesh) (Math|Transform|MakeTransform "0, 0, 0" "0, 0, 0" "1.000000,1.000000,1.000000") false false))))

(fn PureGetReloadInfo
  (Utilities|FlowControl|Sequence
    (:then_0
      (bind _output_get (LocalVariables|Setl_AmmoNeeded (- (Variables|Default|GetMaxAmmo) (Variables|Default|GetAmmo))))
      (if (> _output_get 0)
        (LocalVariables|Setl_AmmoIHave (CallFunction|PureGetAmmoinInventory (Variables|Default|GetAmmoID)))))
    (:then_1
      (return (LocalVariables|Getl_AmmoIHave) (LocalVariables|Getl_AmmoNeeded)))))

(fn PureGetAmmoinInventory
  (params (ID :type Name))
  (bind _result (Default|FindItembyID (Variables|/Game/Defend/Blueprints/Pawns/Pawn_L1_Equipment.Pawn_L1_Equipment_C|GetEquipmentInventoryComponent (.AsPawn%20L1%20Equipment (Utilities|Casting|CastToPawn_L1_Equipment (Variables|Default|GetItemOwner)))) ID))
  (for _array_element _result
    (bind _output_get (LocalVariables|Setl_AmmoIHave (+ (.Amount (Utilities|Struct|BreakInventoryItem _array_element)) (stale _output_get)))))
  (return (LocalVariables|Getl_AmmoIHave)))

(fn FunconRecall
  (params (ActionName :type Name) (ActionBegin :type Boolean))
  (switch name ActionName
    (:Pickaxe
      (CallFunction|FuncApplyDamageonTarget))))

(fn IGetAmmoID
  (return (Variables|Default|GetAmmoID)))

(fn IGetAttachType
  (return "NewEnumerator1"))

(fn FuncRepairTarget
  (bind _asplayer_controller (CallFunction|PureGetOwnerPC))
  (bind _itemowner (Variables|Default|GetItemOwner))
  (bind _array (Utilities|Array|MakeArray _itemowner))
  (bind (_hitresult _returnvalue) (Class|CXZFuncLib|CXZLineTracefromScreenPosPercentage _asplayer_controller "TraceTypeQuery1" _array true true 0.5 0.5))
  (bind (_bblockinghit _binitialoverlap _time _distance _location _impactpoint _normal _impactnormal _physmat _hitactor) (Collision|BreakHitResult _hitresult))
  (Utilities|IsValid _asplayer_controller
    (:Is%20Valid
      (if _returnvalue
        (bind _output_get (LocalVariables|Setl_HitLocation _location))
        (Rendering|Debug|DrawDebugSphere _output_get 1e+01 12 "(R=1.000000,G=0.000000,B=0.000000,A=1.000000)" 3.0 1.0)
        (LocalVariables|Setl_HitActor _hitactor)
        (LocalVariables|Setl_HitDistance (Math|Vector|Distance(Vector) (LocalVariables|Getl_HitLocation) (Transformation|GetWorldLocation (Variables|Default|GetStaticMesh))))
        (bind _asvoxel_world (Utilities|Casting|CastToVoxelWorld (LocalVariables|Getl_HitActor))
          (:then
            (LocalVariables|Setl_VoxelWorld _asvoxel_world)
            (if (<= (LocalVariables|Getl_HitDistance) (Variables|Default|GetMaxDistanceVoxel))
              (Class|VoxelSphereTools|RevertSpheretoGenerator (LocalVariables|Getl_VoxelWorld) (LocalVariables|Getl_HitLocation) (Variables|/Script/Voxel.VoxelWorld|GetVoxelSize (LocalVariables|Getl_VoxelWorld)) true true true false)
              (return true)
              (else
                (return false))))
          (:CastFailed
            (return false)))
        (else
          _)))
    (:Is%20Not%20Valid
      _))
  (return false))

(fn FuncAddtoTarget
  (bind _asplayer_controller (CallFunction|PureGetOwnerPC))
  (bind _itemowner (Variables|Default|GetItemOwner))
  (bind _array (Utilities|Array|MakeArray _itemowner))
  (bind (_hitresult _returnvalue) (Class|CXZFuncLib|CXZLineTracefromScreenPosPercentage _asplayer_controller "TraceTypeQuery1" _array true true 0.5 0.5))
  (bind (_bblockinghit _binitialoverlap _time _distance _location _impactpoint _normal _impactnormal _physmat _hitactor) (Collision|BreakHitResult _hitresult))
  (Utilities|IsValid _asplayer_controller
    (:Is%20Valid
      (if _returnvalue
        (bind _output_get (LocalVariables|Setl_HitLocation _location))
        (Rendering|Debug|DrawDebugSphere _output_get 1e+01 12 "(R=1.000000,G=0.000000,B=0.000000,A=1.000000)" 3.0 1.0)
        (LocalVariables|Setl_HitActor _hitactor)
        (LocalVariables|Setl_HitDistance (Math|Vector|Distance(Vector) (LocalVariables|Getl_HitLocation) (Transformation|GetWorldLocation (Variables|Default|GetStaticMesh))))
        (bind _asvoxel_world (Utilities|Casting|CastToVoxelWorld (LocalVariables|Getl_HitActor))
          (:then
            (LocalVariables|Setl_VoxelWorld _asvoxel_world)
            (if (<= (LocalVariables|Getl_HitDistance) (Variables|Default|GetMaxDistanceVoxel))
              (Class|VoxelSphereTools|AddSphere (LocalVariables|Getl_VoxelWorld) (LocalVariables|Getl_HitLocation) (Variables|/Script/Voxel.VoxelWorld|GetVoxelSize (LocalVariables|Getl_VoxelWorld)))
              (return true)
              (else
                (return false))))
          (:CastFailed
            (return false)))
        (else
          _)))
    (:Is%20Not%20Valid
      _))
  (return false))

(fn FuncReportMining
  (params (ModifiedValues :type Array%20of%20Modified%20Voxel%20Value%20Structures) (EditedBounds :type Voxel%20Int%20Box%20Structure) (Who :type Actor%20Object%20Reference) (VWorld :type Voxel%20World%20Object%20Reference))
  (bind _outactors (Actor|GetAllActorsOfClass "/Game/Defend/Voxel/BP_VoxelMining.BP_VoxelMining_C"))
  (if (> (Utilities|Array|Length _outactors) 0)
    (Default|CEVoxelMined (Utilities|Array|Get(acopy) _outactors) ModifiedValues EditedBounds Who VWorld)))

(fn IGetInteractDistance
  (return 2.5e+02))