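; BP_Ring_Spike is an equipable spike ring item actor that relies on its parent Blueprint for most behavior.
; It extends the parent drop function to triple the skeletal mesh scale, and the pickup interface event restores normal scale.
; The equip event is empty, and leftover nodes that hide the actor and destroy its mesh are disconnected.
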(event EventBeginPlay
  (|CallParentFunction))

(event Collision|EventActorBeginOverlap
  (params (OtherActor :type Actor%20Object%20Reference))
  (|CallParentFunction OtherActor) ; This node is disabled and will not be called.\nDrag off pins to build functionality.
)

(event EventTick
  (params (DeltaSeconds :type Float%20%28single-precision%29))
  (|CallParentFunction DeltaSeconds) ; This node is disabled and will not be called.\nDrag off pins to build functionality.
)

(event EventIPickup
  (params (Who :type Actor%20Object%20Reference))
  (Transformation|SetRelativeScale3D (Variables|Default|GetSkeletalMesh) "1.000000,1.000000,1.000000"))

(event EventIEquiped
  (params (Who :type Pawn%20L1%20Equipment%20Object%20Reference)))

(fn ConstructionScript
  (|CallParentFunction))

(fn FuncDrop
  (|CallParentFunction)
  (Transformation|SetRelativeScale3D (Variables|Default|GetSkeletalMesh) "3.000000,3.000000,3.000000"))