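; Equipable backpack item actor that carries its own inventory of BagSize slots and extends the wearer's inventory while worn.
; Equipping enlarges the wearer's inventory, moves the bag's items into it in reverse slot order and offers them to the hotbar.
; Unequipping shrinks it slot by slot, moving items from removed slots back into the bag.
; For equipment pawns, using a non-empty bag requires a free matching equipment slot.
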(event EventBeginPlay
  (|CallParentFunction)
  (Default|ServerInitInventory (Variables|Default|GetInventoryComponent) (Variables|Default|GetBagSize)))

(event Collision|EventActorBeginOverlap
  (params (OtherActor :type Actor%20Object%20Reference))
  (|CallParentFunction OtherActor) ; This node is disabled and will not be called.\nDrag off pins to build functionality.
)

(event EventTick
  (params (DeltaSeconds :type Float%20%28single-precision%29))
  (|CallParentFunction DeltaSeconds) ; This node is disabled and will not be called.\nDrag off pins to build functionality.
)

(event EventIEquiped
  (params (Who :type Pawn%20L1%20Equipment%20Object%20Reference))
  (CallFunction|FuncEquiped Who))

(event EventIUnequiped
  (params (Who :type Pawn%20L1%20Equipment%20Object%20Reference))
  (CallFunction|FuncUnequiped Who))

(fn ConstructionScript
  (|CallParentFunction))

(fn FuncEquiped
  (params (Who :type Pawn%20L1%20Equipment%20Object%20Reference))
  (bind _inventorymanagercomponent (Variables|/Game/Defend/Blueprints/Pawns/Pawn_L1_Equipment.Pawn_L1_Equipment_C|GetInventoryManagerComponent Who))
  (Development|PrintString (Utilities|String|Append (Utilities|String|ToString(Integer) (Variables|Default|GetBagSize)) "格背包装备") true true "(R=0.098097,G=1.000000,B=0.000000,A=1.000000)" 2.1e+02)
  (Default|ServerIncreaseInventorySize (Variables|/Game/Defend/Blueprints/Pawns/Pawn_L1_Equipment.Pawn_L1_Equipment_C|GetInventoryManagerComponent Who) (Variables|Default|GetBagSize))
  (for _index (range 0 (- (Variables|Default|GetBagSize) 1))
    (bind _inventoryitem (Default|GetInventoryItem (Variables|Default|GetInventoryComponent) _index))
    (Utilities|IsValid (.Icon (Utilities|Struct|BreakInventoryItem _inventoryitem))
      (:Is%20Valid
        (Default|AddItem _inventorymanagercomponent (Variables|/Game/Defend/Blueprints/Pawns/Pawn_L1_Equipment.Pawn_L1_Equipment_C|GetEquipmentInventoryComponent Who) (- (+ (Variables|/Game/Defend/Blueprints/Components/InventoryManagerComponent.InventoryManagerComponent_C|GetInventorySize _inventorymanagercomponent) 13) _index) _inventoryitem)
        (Default|CETrytoHotbarwhenPickup Who _inventoryitem)
        (Utilities|Array|SetArrayElem :TargetArray (Variables|/Game/Defend/Blueprints/Components/InventoryComponent.InventoryComponent_C|GetInventory (Variables|Default|GetInventoryComponent)) :Index _index)))))

(fn FuncUnequiped
  (params (Who :type Pawn%20L1%20Equipment%20Object%20Reference))
  (bind _inventorymanagercomponent (Variables|/Game/Defend/Blueprints/Pawns/Pawn_L1_Equipment.Pawn_L1_Equipment_C|GetInventoryManagerComponent Who))
  (Development|PrintString (Utilities|String|Append (Utilities|String|ToString(Integer) (Variables|Default|GetBagSize)) "格背包卸下") true true "(R=0.635417,G=0.564999,B=0.000000,A=1.000000)" 2.1e+02)
  (for _index (range 0 (- (Variables|Default|GetBagSize) 1))
    (LocalVariables|Setl_CurIdx _index)
    (bind _needtoremoveitem (Default|DecreaseInventorySize _inventorymanagercomponent (Variables|/Game/Defend/Blueprints/Pawns/Pawn_L1_Equipment.Pawn_L1_Equipment_C|GetEquipmentInventoryComponent Who) 1))
    (if _needtoremoveitem
      (Default|MoveItem (Variables|/Game/Defend/Blueprints/Pawns/Pawn_L1_Equipment.Pawn_L1_Equipment_C|GetInventoryManagerComponent Who) (Variables|/Game/Defend/Blueprints/Pawns/Pawn_L1_Equipment.Pawn_L1_Equipment_C|GetEquipmentInventoryComponent Who) (+ (Variables|/Game/Defend/Blueprints/Components/InventoryManagerComponent.InventoryManagerComponent_C|GetInventorySize _inventorymanagercomponent) 13) (Variables|Default|GetInventoryComponent) (LocalVariables|Getl_CurIdx))
      (bind _needtoremoveitem_2 (Default|DecreaseInventorySize (Variables|/Game/Defend/Blueprints/Pawns/Pawn_L1_Equipment.Pawn_L1_Equipment_C|GetInventoryManagerComponent Who) (Variables|/Game/Defend/Blueprints/Pawns/Pawn_L1_Equipment.Pawn_L1_Equipment_C|GetEquipmentInventoryComponent Who) 1))
      (if _needtoremoveitem_2
        (Development|PrintString "err")))))

(fn OnActorUsed
  (params (Pawn :type Pawn%20Object%20Reference))
  (bind _itemcount (Default|GetInventoryItemCount (Variables|Default|GetInventoryComponent)))
  (if (> _itemcount 0)
    (bind _aspawn_l1_equipment (Utilities|Casting|CastToPawn_L1_Equipment Pawn)
      (:then
        (bind _hasemptyslot (Default|GetEmptyEquipmentSlotbyType (Variables|/Game/Defend/Blueprints/Pawns/Pawn_L1_Equipment.Pawn_L1_Equipment_C|GetInventoryManagerComponent _aspawn_l1_equipment) "NewEnumerator5"))
        (if _hasemptyslot
          (bind _success (|CallParentFunction Pawn))
          (return _success)
          (else
            (return false))))
      (:CastFailed
        _)))
  (bind _success_2 (|CallParentFunction Pawn))
  (return _success_2))

(fn IGetSize
  (return (Variables|Default|GetBagSize)))

(fn IIsEmpty
  (bind _itemcount (Default|GetInventoryItemCount (Variables|Default|GetInventoryComponent)))
  (return (== _itemcount 0)))