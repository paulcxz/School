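; BP_CXZItem is an item actor that characters can pick up and drop, with an empty interaction hook.
; Interface events route to overridable-style functions: pickup locks the item, records and notifies its owner, and copies the owner's team ID, defaulting to -1.
; Drop clears the owner, re-enables pickup, physics and collision on both meshes, and detaches the root in world space.
; It also exposes its overlay state and owning PlayerController.
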(event EventIPickup
  (params (Who :type Actor%20Object%20Reference))
  (CallFunction|FuncPickup Who))

(event EventIDrop
  (CallFunction|FuncDrop))

(event EventIInteract
  (params (Who :type Actor%20Object%20Reference))
  (CallFunction|FuncBeenInteracted Who))

(fn ConstructionScript)

(fn PureGetOwnerPC
  (bind _aspawn (Utilities|Casting|CastToPawn (Variables|Default|GetItemOwner))
    (:then
      (bind _asplayer_controller (Utilities|Casting|CastToPlayerController (Pawn|GetController _aspawn))
        (:then
          (return _asplayer_controller))
        (:CastFailed
          _)))
    (:CastFailed
      _))
  (return 0))

(fn FuncBeenInteracted
  (params (ByWhom :type Actor%20Object%20Reference)))

(fn FuncPickup
  (params (ByWhom :type Actor%20Object%20Reference))
  (if (Variables|Default|GetPickupable)
    (Variables|Default|SetPickupable false)
    (bind _output_get (Variables|Default|SetItemOwner ByWhom))
    (Class|IItemContainer|IGetItem(Message) _output_get self)
    (if (Utilities|DoesObjectImplementInterface (Variables|Default|GetItemOwner) "/Game/Defend/Blueprints/Interfaces/I_Team.I_Team_C")
      (bind _id (Class|ITeam|IGetTeamID(Message) (Variables|Default|GetItemOwner)))
      (Variables|Default|SetTeamID _id)
      (else
        (Variables|Default|SetTeamID -1)))))

(fn FuncDrop
  (bind _skeletalmesh (Variables|Default|GetSkeletalMesh))
  (bind _staticmesh (Variables|Default|GetStaticMesh))
  (Variables|Default|SetItemOwner 0)
  (Variables|Default|SetPickupable true)
  (Physics|SetSimulatePhysics _skeletalmesh true)
  (Collision|SetCollisionEnabled _skeletalmesh "QueryAndPhysics")
  (Physics|SetSimulatePhysics _staticmesh true)
  (Collision|SetCollisionEnabled _staticmesh "QueryAndPhysics")
  (Transformation|DetachFromComponent (Variables|Default|GetRoot) "KeepWorld" "KeepWorld" "KeepWorld" true))

(fn IGetInteractDistance
  (return 0.0))

(fn IGetOverlayState
  (return (Variables|Default|GetOverlayState)))