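; Enemy spawner that runs escalating waves of Pawn_L4_Enemy at its scene component's location.
; Each level-up, on BeginPlay and after waves, raises the cumulative spawn target by an amount scaled to the level.
; Tick attempts one spawn per frame until the target is met, counting only valid spawns so collision-blocked attempts retry.
; Each enemy's death event feeds a kill counter that, on reaching the target, triggers the next level after a short delay.
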(event Custom|CE_LevelUp
  (bind _level (Variables|Default|GetLevel))
  (Math|Integer|IncrementInt _level
    (:%20%20
      (bind _output_get (Variables|Default|SetEnemiesToSpawn (+ (stale _output_get) (* _level 6)))))))

(event Custom|BE_OneDead
  (Math|Integer|IncrementInt (Variables|Default|GetEnemyDied)
    (:%20%20
      (if (>= (Variables|Default|GetEnemyDied) (Variables|Default|GetEnemiesToSpawn))
        (Utilities|FlowControl|Delay 3.0)
        (CallFunction|CELevelUp)))))

(event EventBeginPlay
  (CallFunction|CELevelUp))

(event EventTick
  (params (DeltaSeconds :type Float%20%28single-precision%29))
  (if (> (Variables|Default|GetEnemiesToSpawn) (Variables|Default|GetEnemySpawned))
    (bind _returnvalue (Game|SpawnActorfromClass "/Game/Defend/Blueprints/Pawns/Pawn_L4_Enemy.Pawn_L4_Enemy_C" (Math|Transform|MakeTransform (Transformation|GetWorldLocation (Variables|Default|GetScene)) "0, 0, 0" "1,1,1") "AdjustIfPossibleButDontSpawnIfColliding" 0 0.0 0))
    (Utilities|IsValid _returnvalue
      (:Is%20Valid
        (Math|Integer|IncrementInt (Variables|Default|GetEnemySpawned)
          (:%20%20
            (EventDispatchers|BindEventtoEDDead _returnvalue (delegate Custom|BE_OneDead))))))))

(fn ConstructionScript)